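; Player 1 slime character, with movement, zoom and pause input, that grows by scoring from grass and enemies.
; AddScore functions rescale the mesh from Score and copy it to the GameInstance.
; AddItem grants Wolf dash, Wisp flash or WingRabbit high-jump abilities, fired alongside Explosion by the Ability input.
; Jumping uses timers to deduct score and spawn AI split slimes; touching a larger BP_Character_02 opens the result level.
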(event OnComponentBeginOverlap(Sphere)
  (params (OverlappedComponent :type Primitive%20Component%20Object%20Reference) (OtherActor :type Actor%20Object%20Reference) (OtherComp :type Primitive%20Component%20Object%20Reference) (OtherBodyIndex :type Integer) (bFromSweep :type Boolean) (SweepResult :type Hit%20Result%20Structure%20%28by%20ref%29))
  (bind _returnvalue (Game|GetPlayerCharacter 1))
  (bind _asbp_character_02 (Utilities|Casting|CastToBP_Character_02 _returnvalue))
  ;[1 1 1] SlimeBattle
  (if (.bSuccess (Utilities|Casting|CastToBP_Character_02 OtherActor))
    (Utilities|FlowControl|Sequence ; Player追加ここ
      (:then_0
        (bind _output_get (Variables|Default|SetSlimeScale (.z (Transformation|GetWorldScale (Variables|Character|GetMesh))))))
      (:then_1
        (bind _output_get_2 (Variables|/Game/BluePrints/BP_Character/BP_Character_02.BP_Character_02_C|SetSlimeScale_2 _asbp_character_02 (.z (Transformation|GetWorldScale (Variables|/Script/Engine.Character|GetMesh _asbp_character_02)))))))
    (if (< _output_get _output_get_2)
      ;;[1 1 1] イベント中に相手に触れるとスコアup
      (CallFunction|CatchRun)
      (Game|OpenLevel(byName) "result"))))

(event Custom|catchRun
  ;[1 1 1] 追いかけっこイベント
  (Utilities|FlowControl|Sequence
    (:then_0
      (Utilities|FlowControl|Delay 6e+01)
      (bind _output_get (Variables|Default|SetScore (Math|Float|Truncate (* (+ (Variables|Default|GetScore) (Variables|/Game/BluePrints/BP_Character/BP_Character_02.BP_Character_02_C|GetScore (.AsBP%20Character%2002 (Utilities|Casting|CastToBP_Character_02 (Game|GetPlayerCharacter 1))))) 1.3)))))))

(event EventBeginPlay
  ;[1 1 1] Score,Enlargement
  (Utilities|FlowControl|Sequence ; 敵のスコア/スライムの巨大化数値
    (:then_0
      (Variables|Default|Setscore_slime 1) ; 草のスコア
      (Variables|Default|SetScoreWisp 20) ; Wispのスコア
      (Variables|Default|SetScoreLizard 10) ; Lizardのスコア
      (Variables|Default|SetScoreWingRabbit 30)
      (Variables|Default|Setscore_wolf 40) ; ウルフのスコア/新しい敵はこの右に継ぎ足しok
    )
    (:then_1
      (Variables|Default|Setmagnification_score 80) ; スライムの大きくなるscoreの設定
      (Variables|Default|Setmagnification 0.2) ; スライムの大きくなる倍率
      (Variables|Default|Setmagnification_vector "1.000000,1.000000,1.000000") ; 巨大化に使うVector値。いじらなくてヨシ!
    )))

(event Input|ActionEvents|InputActionJump
  (params (Key :type Key%20Structure :default "None"))
  ;[1 1 1] Controller
  (:Pressed
    (Utilities|Time|SetTimerbyFunctionName 0 "Jump" 0.5)
    (Utilities|Time|SetTimerbyFunctionName 0 "JumpUseScore" 2.0)
    (Utilities|Time|SetTimerbyFunctionName 0 "SplitSlime" 2.0)))

(event Input|ActionEvents|InputActionPause
  (params (Key :type Key%20Structure :default "None"))
  ;[1 1 1] ホーム画面押したらポーズ画面表示
  (:Pressed
    (bind _returnvalue (UserInterface|CreateWidget "/Game/pause/pause_UI.pause_UI_C"))
    (UserInterface|Viewport|AddtoViewport _returnvalue 0)
    (Variables|/Script/Engine.PlayerController|SetbShowMouseCursor (Game|GetPlayerController 0) true)
    (Game|SetGamePaused true)))

(event Input|ActionEvents|InputActionAbility
  (params (Key :type Key%20Structure :default "None"))
  (bind _returnvalue (Game|GetPlayerCharacter 0))
  (bind _mesh (Variables|Character|GetMesh))
  (bind _returnvalue_2 (Transformation|GetActorLocation _returnvalue))
  ;[1 1 1] Ability
  (:Pressed
    (Audio|PlaySoundatLocation "/Game/Sounds/04_Slime_Activate.04_Slime_Activate" _returnvalue_2 "0, 0, 0" 1.0 1.0 0.0 "/Game/Sounds/NewSoundAttenuation.NewSoundAttenuation" 0 0) ; Slime_Activate
    (Utilities|FlowControl|Sequence
      (:then_0
        (if (Variables|Default|GetWolfAbility)
          (CallFunction|SetWolf)
          (Audio|PlaySoundatLocation "/Game/Sounds/11_SlimeWolf_Dash_2.11_SlimeWolf_Dash_2" _returnvalue_2 "0, 0, 0" 1.0 1.0 0.0 "/Game/Sounds/NewSoundAttenuation.NewSoundAttenuation" 0 0) ; SlimeWolf_Dash
          (Utilities|Time|SetTimerbyFunctionName 0 "AbilityWalkSpeed" 3.0)
          (Variables|Default|SetWolfAbility false)
          (Variables|Default|SetHaveItem? false :!label _label)))
      (:then_1
        (if (Variables|Default|GetWispAbility)
          (CallFunction|SetWisp)
          (Audio|PlaySoundatLocation "/Game/Sounds/12_SlimeWisp_FlashAttack.12_SlimeWisp_FlashAttack" (Transformation|GetActorLocation (Game|GetPlayerCharacter 0)) "0, 0, 0" 1.0 1.0 0.0 "/Game/Sounds/NewSoundAttenuation.NewSoundAttenuation" 0 0) ; SlimeWisp_FlashAttack
          (Variables|Default|SetWispAbility false)
          (goto _label)))
      (:then_2
        (if (Variables|Default|GetWingRabitAbility)
          (Components|Movement|StopMovementImmediately (Variables|Character|GetCharacterMovement))
          (Audio|PlaySoundatLocation "/Game/Sounds/13_SlimeWing_Rise_short.13_SlimeWing_Rise_short" _returnvalue_2 "0, 0, 0" 1.0 1.0 0.0 "/Game/Sounds/NewSoundAttenuation.NewSoundAttenuation" 0 0) ; SlimeWing_Rise
          (CallFunction|SetWingRabbit)
          (Utilities|Time|SetTimerbyFunctionName 0 "AbilityJumpStetas" 0.1)
          (Variables|Default|SetWingRabitAbility false)
          (Utilities|FlowControl|Sequence
            (:then_0
              (goto _label))
            (:then_1
              (Utilities|Time|SetTimerbyFunctionName 0 "WingRabbitSound" 2.0)))))
      (:then_3
        (if (Variables|Default|GetExplosionAbility)
          (Game|SpawnActorfromClass "/Game/expeffect/EffectExplosion.EffectExplosion_C" (Math|Transform|MakeTransform (+ (Transformation|GetWorldLocation _mesh) "0, 0,5.000000") "0, 0, 0" (+ (Transformation|GetWorldScale _mesh) "5.000000,5.000000,5.000000")) "Undefined" 0 0)
          (Audio|PlaySoundatLocation 0 _returnvalue_2 "0, 0, 0" 1.0 1.0 0.0 0 0 0)
          (Variables|Default|SetExplosionAbility false)
          (goto _label))))))

(event Input|AxisEvents|InputAxisMoveForward
  (params (AxisValue :type Float%20%28single-precision%29))
  (bind _returnvalue (Game|Player|GetPlayerPawn 0))
  ;[1 1 1] Controller
  (Pawn|Input|AddMovementInput _returnvalue (Math|Vector|GetForwardVector (Pawn|GetControlRotation _returnvalue :!class /Script/Engine.Pawn)) AxisValue false))

(event Input|AxisEvents|InputAxisMoveRight
  (params (AxisValue :type Float%20%28single-precision%29))
  (bind _returnvalue (Game|Player|GetPlayerPawn 0))
  ;[1 1 1] Controller
  (Pawn|Input|AddMovementInput _returnvalue (Math|Vector|GetRightVector (Pawn|GetControlRotation _returnvalue :!class /Script/Engine.Pawn)) AxisValue false))

(event Input|AxisEvents|InputAxisForcus
  (params (AxisValue :type Float%20%28single-precision%29))
  (bind _springarm (Variables|Default|GetSpringArm))
  ;[1 1 1] Comment
  (Variables|/Script/Engine.SpringArmComponent|SetTargetArmLength _springarm (+ (Variables|/Script/Engine.SpringArmComponent|GetTargetArmLength _springarm) (* AxisValue -1e+01))))

(event Input|AxisEvents|InputAxisTurn
  (params (AxisValue :type Float%20%28single-precision%29))
  ;[1 1 1] Controller
  (Pawn|Input|AddControllerYawInput (Game|GetPlayerCharacter 0) AxisValue))

(fn ConstructionScript)

(fn AddScore
  (bind _output_get (Variables|Default|SetScore (+ (Variables|Default|GetScore) (Variables|Default|Getscore_slime))))
  (Variables|Default|SetAddScore? true)
  (Variables|Default|SetAddScoreRabbit? false)
  (Variables|Default|SetAddScoreWisp? false)
  (Variables|Default|SetAddScoreLizard? false)
  (Variables|Default|SetAddScoreWolf? false)
  (Variables|Default|SetAddScoreSplitSlime? false)
  (Transformation|SetWorldScale3D (Variables|Character|GetMesh) (+ (Variables|Default|Getmagnification_vector) (* (/ _output_get (Variables|Default|Getmagnification_score)) (Variables|Default|Getmagnification))))
  (bind _asgame_instace_bp (Utilities|Casting|CastToGameInstace_BP (Game|GetGameInstance)))
  (Variables|/Game/BluePrints/BP_Wiedget/GameInstace_BP.GameInstace_BP_C|Setslime_1_score _asgame_instace_bp (Variables|Default|GetScore))
  (Utilities|Time|SetTimerbyFunctionName 0 "AddTime" (Variables|Default|GetAddScoreTime)))

(fn SetWingRabbit
  (Variables|/Script/Engine.CharacterMovementComponent|SetJumpZVelocity (Variables|Character|GetCharacterMovement) 1.6e+03)
  (Character|Jump (Game|GetPlayerCharacter 0)))

(fn AddScoreLizard
  (params (Enemy :type Character%20Object%20Reference))
  (bind _asbp_lizard (Utilities|Casting|CastToBP_Lizard Enemy))
  (if (Math|Vector|Equal(Vector) (Transformation|GetActorScale3D _asbp_lizard) "1.000000,1.000000,1.000000" 0.0001)
    (bind _output_get (Variables|Default|SetScore (+ (Variables|Default|GetScore) (Variables|Default|GetScoreLizard))))
    (Transformation|SetWorldScale3D (Variables|Character|GetMesh) (+ (Variables|Default|Getmagnification_vector) (* (/ _output_get (Variables|Default|Getmagnification_score)) (Variables|Default|Getmagnification))))
    (else
      (bind _output_get_2 (Variables|Default|SetScore (+ (Variables|Default|GetScore) (Math|Float|Truncate (* (Variables|Default|GetScoreLizard) (Variables|/Game/Goto/Event/Event_BigScale.Event_BigScale_C|Getmagnification (Variables|Default|GetEventBig)))))))
      (Transformation|SetWorldScale3D (Variables|Character|GetMesh) (+ (Variables|Default|Getmagnification_vector) (* (/ _output_get_2 (Variables|Default|Getmagnification_score)) (Variables|Default|Getmagnification))))))
  (bind _asgame_instace_bp (Utilities|Casting|CastToGameInstace_BP (Game|GetGameInstance)))
  (Variables|/Game/BluePrints/BP_Wiedget/GameInstace_BP.GameInstace_BP_C|Setslime_1_score _asgame_instace_bp (Variables|Default|GetScore))
  (Utilities|Time|SetTimerbyFunctionName 0 "AddLizzerdTime" (Variables|Default|GetAddScoreTime)))

(fn AddScoreWolf
  (params (Enemy :type Character%20Object%20Reference))
  (bind _asbp_wolf (Utilities|Casting|CastToBP_Wolf Enemy))
  (if (Math|Vector|Equal(Vector) (Transformation|GetActorScale3D _asbp_wolf) "1.000000,1.000000,1.000000" 0.0001)
    (bind _output_get (Variables|Default|SetScore (+ (Variables|Default|GetScore) (Variables|Default|Getscore_wolf))))
    (Transformation|SetWorldScale3D (Variables|Character|GetMesh) (+ (Variables|Default|Getmagnification_vector) (* (/ _output_get (Variables|Default|Getmagnification_score)) (Variables|Default|Getmagnification))))
    (else
      (bind _output_get_2 (Variables|Default|SetScore (+ (Variables|Default|GetScore) (Math|Float|Truncate (* (Variables|Default|Getscore_wolf) (Variables|/Game/Goto/Event/Event_BigScale.Event_BigScale_C|Getmagnification (Variables|Default|GetEventBig)))))))
      (Transformation|SetWorldScale3D (Variables|Character|GetMesh) (+ (Variables|Default|Getmagnification_vector) (* (/ _output_get_2 (Variables|Default|Getmagnification_score)) (Variables|Default|Getmagnification))))))
  (bind _asgame_instace_bp (Utilities|Casting|CastToGameInstace_BP (Game|GetGameInstance)))
  (Variables|/Game/BluePrints/BP_Wiedget/GameInstace_BP.GameInstace_BP_C|Setslime_1_score _asgame_instace_bp (Variables|Default|GetScore))
  (Audio|PlaySoundatLocation "/Game/Sounds/03_Slime_Acquired.03_Slime_Acquired" (Transformation|GetActorLocation (Game|GetPlayerCharacter 0)) "0, 0, 0" 1.0 1.0 0.0 "/Game/Sounds/NewSoundAttenuation.NewSoundAttenuation" 0 0)
  (Utilities|Time|SetTimerbyFunctionName 0 "AddWolfTime" (Variables|Default|GetAddScoreTime)))

(fn AddScoreWisp
  (params (Enemy :type Character%20Object%20Reference))
  (bind _asbp_whisp (Utilities|Casting|CastToBP_Whisp Enemy))
  (if (Math|Vector|Equal(Vector) (Transformation|GetActorScale3D _asbp_whisp) "1.000000,1.000000,1.000000" 0.0001)
    (bind _output_get (Variables|Default|SetScore (+ (Variables|Default|GetScore) (Variables|Default|GetScoreWisp))))
    (Transformation|SetWorldScale3D (Variables|Character|GetMesh) (+ (Variables|Default|Getmagnification_vector) (* (/ _output_get (Variables|Default|Getmagnification_score)) (Variables|Default|Getmagnification))))
    (else
      (bind _output_get_2 (Variables|Default|SetScore (+ (Variables|Default|GetScore) (Math|Float|Truncate (* (Variables|Default|GetScoreWisp) (Variables|/Game/Goto/Event/Event_BigScale.Event_BigScale_C|Getmagnification (Variables|Default|GetEventBig)))))))
      (Transformation|SetWorldScale3D (Variables|Character|GetMesh) (+ (Variables|Default|Getmagnification_vector) (* (/ _output_get_2 (Variables|Default|Getmagnification_score)) (Variables|Default|Getmagnification))))))
  (bind _asgame_instace_bp (Utilities|Casting|CastToGameInstace_BP (Game|GetGameInstance)))
  (Variables|/Game/BluePrints/BP_Wiedget/GameInstace_BP.GameInstace_BP_C|Setslime_1_score _asgame_instace_bp (Variables|Default|GetScore))
  (Audio|PlaySoundatLocation "/Game/Sounds/03_Slime_Acquired.03_Slime_Acquired" (Transformation|GetActorLocation (Game|GetPlayerCharacter 0)) "0, 0, 0" 1.0 1.0 0.0 "/Game/Sounds/NewSoundAttenuation.NewSoundAttenuation" 0 0)
  (Utilities|Time|SetTimerbyFunctionName 0 "AddWispTime" (Variables|Default|GetAddScoreTime)))

(fn SetWolf
  (Variables|/Script/Engine.CharacterMovementComponent|SetMaxWalkSpeed (Variables|Character|GetCharacterMovement) (Variables|Default|Getspeed))
  (return))

(fn SetWisp
  (Effects|SpawnEmitteratLocation "/Game/Perticle/WhispParticle1.WhispParticle1" (Transformation|GetWorldLocation (Variables|/Game/BluePrints/BP_Character/BP_Character_02.BP_Character_02_C|GetCamera (.AsBP%20Character%2002 (Utilities|Casting|CastToBP_Character_02 (Game|GetPlayerCharacter 1)))))))

(fn AddScoreWingRabbit
  (params (Enemy :type Character%20Object%20Reference))
  (bind _aswing_rabbit (Utilities|Casting|CastToWingRabbit Enemy))
  (if (Math|Vector|Equal(Vector) (Transformation|GetActorScale3D _aswing_rabbit) "1.000000,1.000000,1.000000" 0.0001)
    (bind _output_get (Variables|Default|SetScore (+ (Variables|Default|GetScore) (Variables|Default|GetScoreWingRabbit))))
    (Transformation|SetWorldScale3D (Variables|Character|GetMesh) (+ (Variables|Default|Getmagnification_vector) (* (/ _output_get (Variables|Default|Getmagnification_score)) (Variables|Default|Getmagnification))))
    (else
      (bind _output_get_2 (Variables|Default|SetScore (+ (Variables|Default|GetScore) (Math|Float|Truncate (* (Variables|Default|GetScoreWingRabbit) (Variables|/Game/Goto/Event/Event_BigScale.Event_BigScale_C|Getmagnification (Variables|Default|GetEventBig)))))))
      (Transformation|SetWorldScale3D (Variables|Character|GetMesh) (+ (Variables|Default|Getmagnification_vector) (* (/ _output_get_2 (Variables|Default|Getmagnification_score)) (Variables|Default|Getmagnification))))))
  (bind _asgame_instace_bp (Utilities|Casting|CastToGameInstace_BP (Game|GetGameInstance)))
  (Variables|/Game/BluePrints/BP_Wiedget/GameInstace_BP.GameInstace_BP_C|Setslime_1_score _asgame_instace_bp (Variables|Default|GetScore))
  (Audio|PlaySoundatLocation "/Game/Sounds/03_Slime_Acquired.03_Slime_Acquired" (Transformation|GetActorLocation (Game|GetPlayerCharacter 0)) "0, 0, 0" 1.0 1.0 0.0 "/Game/Sounds/NewSoundAttenuation.NewSoundAttenuation" 0 0)
  (Utilities|Time|SetTimerbyFunctionName 0 "AddRabbitTime" (Variables|Default|GetAddScoreTime)))

(fn AddItem
  (bind _actortrace (Variables|Default|GetActorTrace))
  (bind _actortrace_2 (Variables|Default|GetActorTrace))
  (bind (_asbp_wolf _bsuccess) (Utilities|Casting|CastToBP_Wolf _actortrace))
  (bind (_aswing_rabbit _bsuccess_2) (Utilities|Casting|CastToWingRabbit _actortrace))
  (bind (_asbp_whisp _bsuccess_3) (Utilities|Casting|CastToBP_Whisp _actortrace))
  (bind (_aswing_rabbit_2 _bsuccess_4) (Utilities|Casting|CastToWingRabbit _actortrace_2))
  (bind (_asbp_wolf_2 _bsuccess_5) (Utilities|Casting|CastToBP_Wolf _actortrace_2))
  (bind (_asbp_whisp_2 _bsuccess_6) (Utilities|Casting|CastToBP_Whisp _actortrace_2))
  (if (Variables|Default|GetHaveItem?)
    (Variables|Default|SetWispAbility false)
    (Variables|Default|SetWolfAbility false)
    (Variables|Default|SetWingRabitAbility false)
    (Utilities|FlowControl|Sequence
      (:then_0
        (if _bsuccess
          (Utilities|Array|Add (Variables|Default|GetInventory) (Variables|/Game/BluePrints/BP_Inventory/Inventory/test.test_C|GetItemData _asbp_wolf))
          (Variables|Default|SetWolfAbility true)
          (Variables|Default|SetHaveItem? true :!label _label)
          (return)))
      (:then_1
        (if _bsuccess_3
          (Utilities|Array|Add (Variables|Default|GetInventory) (Variables|/Game/BluePrints/BP_Inventory/Inventory/test.test_C|GetItemData _asbp_whisp))
          (Variables|Default|SetWispAbility true)
          (goto _label)))
      (:then_2
        (if _bsuccess_2
          (Utilities|Array|Add (Variables|Default|GetInventory) (Variables|/Game/BluePrints/BP_Inventory/Inventory/test.test_C|GetItemData _aswing_rabbit))
          (Variables|Default|SetWingRabitAbility true)
          (goto _label))))
    (else
      (Utilities|FlowControl|Sequence
        (:then_0
          (if _bsuccess_5
            (Utilities|Array|Add (Variables|Default|GetInventory) (Variables|/Game/BluePrints/BP_Inventory/Inventory/test.test_C|GetItemData _asbp_wolf_2))
            (Variables|Default|SetWolfAbility true)
            (Variables|Default|SetHaveItem? true :!label _label_2)
            (return)))
        (:then_1
          (if _bsuccess_6
            (Utilities|Array|Add (Variables|Default|GetInventory) (Variables|/Game/BluePrints/BP_Inventory/Inventory/test.test_C|GetItemData _asbp_whisp_2))
            (Variables|Default|SetWispAbility true)
            (goto _label_2)))
        (:then_2
          (if _bsuccess_4
            (Utilities|Array|Add (Variables|Default|GetInventory) (Variables|/Game/BluePrints/BP_Inventory/Inventory/test.test_C|GetItemData _aswing_rabbit_2))
            (Variables|Default|SetWingRabitAbility true)
            (goto _label_2)))))))

(fn ScoreInstance
  (bind _asgame_instace_bp (Utilities|Casting|CastToGameInstace_BP (Game|GetGameInstance)))
  (Variables|/Game/BluePrints/BP_Wiedget/GameInstace_BP.GameInstace_BP_C|Setslime_1_score _asgame_instace_bp (Variables|Default|GetScore)))

(fn ScoreGameInstance
  (bind _asgame_instace_bp (Utilities|Casting|CastToGameInstace_BP (Game|GetGameInstance)))
  (bind _output_get (Variables|/Game/BluePrints/BP_Wiedget/GameInstace_BP.GameInstace_BP_C|Setslime_1_score _asgame_instace_bp (Variables|Default|GetScore)))
  (Development|PrintText (Utilities|Text|ToText(Integer) _output_get)))

(fn SplitSlime
  (bind _returnvalue (Math|Random|RandomFloatinRange 4e+02 4e+02))
  (bind _returnvalue_2 (Math|Random|RandomFloatinRange -4e+02 4e+02))
  (bind _mesh (Variables|Character|GetMesh))
  (bind _splitslimesize (Variables|Default|GetSplitSlimeSize))
  (bind _returnvalue_3 (Transformation|GetWorldLocation _mesh))
  (bind _returnvalue_4 (Math|Vector|MakeVector _returnvalue _returnvalue_2 0.0))
  (bind _returnvalue_5 (Transformation|GetWorldScale _mesh))
  (bind _returnvalue_6 (Transformation|GetWorldScale _mesh))
  (bind _returnvalue_7 (Math|Random|RandomPointinBoundingBox _returnvalue_3 _returnvalue_4))
  (bind _returnvalue_8 (* _returnvalue_6 _splitslimesize))
  (bind _returnvalue_9 (- _returnvalue_5 _returnvalue_8))
  (bind _returnvalue_10 (Math|Transform|MakeTransform _returnvalue_7 "0, 0, 0" _returnvalue_9))
  (Utilities|FlowControl|Sequence
    (:then_0
      (bind _returnvalue_11 (Game|SpawnActorfromClass "/Game/BluePrints/BP_Character/AI/BP_AICharacter.BP_AICharacter_C" _returnvalue_10 "Undefined" 0 0))
      (Pawn|SpawnDefaultController _returnvalue_11))
    (:then_1
      (bind _returnvalue_12 (Game|SpawnActorfromClass "/Game/BluePrints/BP_Character/AI/BP_AICharacter.BP_AICharacter_C" _returnvalue_10 "Undefined" 0 0))
      (Pawn|SpawnDefaultController _returnvalue_12))))

(fn JumpUseScore
  (Variables|Default|SetScore (- (Variables|Default|GetScore) (Variables|Default|GetJumpScore))))

(fn AbilityWalkSpeed
  (Variables|/Script/Engine.CharacterMovementComponent|SetMaxWalkSpeed (Variables|Character|GetCharacterMovement) 4.2e+02))

(fn AbilityJumpStetas
  (Variables|/Script/Engine.CharacterMovementComponent|SetJumpZVelocity (Variables|Character|GetCharacterMovement) 8e+02))

(fn WingRabbitSound
  (Audio|PlaySoundatLocation "/Game/Sounds/14_SlimeWing_Descent.14_SlimeWing_Descent" (Transformation|GetActorLocation (Game|GetPlayerCharacter 0)) "0, 0, 0" 1.0 1.0 0.0 0 0 0) ; SlimeWing_Descent
)

(fn AddScoreSplitSlime
  (bind _output_get (Variables|Default|SetScore (+ (Variables|Default|GetScore) (Variables|Default|GetScoreSplitSlime))))
  (Variables|Default|SetAddScoreSplitSlime? true)
  (Variables|Default|SetAddScore? false)
  (Variables|Default|SetAddScoreRabbit? false)
  (Variables|Default|SetAddScoreLizard? false)
  (Variables|Default|SetAddScoreWisp? false)
  (Variables|Default|SetAddScoreWolf? false)
  (Transformation|SetWorldScale3D (Variables|Character|GetMesh) (+ (Variables|Default|Getmagnification_vector) (* (/ _output_get (Variables|Default|Getmagnification_score)) (Variables|Default|Getmagnification))))
  (bind _asgame_instace_bp (Utilities|Casting|CastToGameInstace_BP (Game|GetGameInstance)))
  (Variables|/Game/BluePrints/BP_Wiedget/GameInstace_BP.GameInstace_BP_C|Setslime_1_score _asgame_instace_bp (Variables|Default|GetScore))
  (Audio|PlaySoundatLocation "/Game/Sounds/03_Slime_Acquired.03_Slime_Acquired" (Transformation|GetActorLocation (Game|GetPlayerCharacter 0)) "0, 0, 0" 1.0 1.0 0.0 "/Game/Sounds/NewSoundAttenuation.NewSoundAttenuation" 0 0)
  (Utilities|Time|SetTimerbyFunctionName 0 "AddSlimeTime" (Variables|Default|GetAddScoreTime)))

(fn AddTime
  (Variables|Default|SetAddScore? false))

(fn AddWolfTime
  (Variables|Default|SetAddScoreWolf? false))

(fn AddWispTime
  (Variables|Default|SetAddScoreWisp? false))

(fn AddRabbitTime
  (Variables|Default|SetAddScoreRabbit? false))

(fn AddLizzerdTime
  (Variables|Default|SetAddScoreLizard? false))

(fn AddSlimeTime
  (Variables|Default|SetAddScoreSplitSlime? false))

(fn AbilityRisset
  (Utilities|FlowControl|Sequence
    (:then_0
      (Variables|Default|SetHaveItem? false))
    (:then_1
      (Variables|Default|SetWolfAbility false))
    (:then_2
      (Variables|Default|SetWispAbility false))
    (:then_3
      (Variables|Default|SetLizardAbility false))
    (:then_4
      (Variables|Default|SetWingRabitAbility false))
    (:then_5
      (Variables|Default|SetExplosionAbility false))))