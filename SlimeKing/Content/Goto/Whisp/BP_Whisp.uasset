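; BP_Whisp is a wisp pickup that either of two player characters can collect once their score is high enough.
; A Move_z timeline offsets the mesh vertically, while Tick spawns a new particle emitter at its location every frame.
; On sphere overlap, a qualifying BP_Character or BP_Character_02 calls AddScoreWisp.
; The matching player, fetched by index, then receives the wisp ability and item, and the pickup destroys itself.
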(event OnComponentBeginOverlap(Sphere)
  (params (OverlappedComponent :type Primitive%20Component%20Object%20Reference) (OtherActor :type Actor%20Object%20Reference) (OtherComp :type Primitive%20Component%20Object%20Reference) (OtherBodyIndex :type Integer) (bFromSweep :type Boolean) (SweepResult :type Hit%20Result%20Structure%20%28by%20ref%29))
  (bind _hitactor (Collision|BreakHitResult SweepResult))
  (bind (_asbp_character _bsuccess) (Utilities|Casting|CastToBP_Character OtherActor))
  (bind (_asbp_character_02 _bsuccess_2) (Utilities|Casting|CastToBP_Character_02 OtherActor))
  (Utilities|FlowControl|Sequence
    (:then_0
      (if _bsuccess
        (if (>= (Variables|/Game/BluePrints/BP_Character/BP_Character.BP_Character_C|GetScore _asbp_character) 20)
          (Default|AddScoreWisp _asbp_character)
          (bind _asbp_character_2 (Utilities|Casting|CastToBP_Character (Game|GetPlayerCharacter 0)))
          (Variables|/Game/BluePrints/BP_Character/BP_Character.BP_Character_C|SetActorTrace _asbp_character_2 _hitactor)
          (Variables|/Game/BluePrints/BP_Character/BP_Character.BP_Character_C|SetWispAbility _asbp_character_2 true)
          (Default|AddItem _asbp_character_2)
          (Actor|DestroyActor :!label _label))))
    (:then_1
      (if _bsuccess_2
        (if (>= (Variables|/Game/BluePrints/BP_Character/BP_Character_02.BP_Character_02_C|GetScore _asbp_character_02) 20)
          (Default|AddScoreWisp _asbp_character_02)
          (bind _asbp_character_02_2 (Utilities|Casting|CastToBP_Character_02 (Game|GetPlayerCharacter 1)))
          (Variables|/Game/BluePrints/BP_Character/BP_Character_02.BP_Character_02_C|SetActorTrace _asbp_character_02_2 _hitactor)
          (Variables|/Game/BluePrints/BP_Character/BP_Character_02.BP_Character_02_C|SetWispAbility2 _asbp_character_02_2 true)
          (Default|AddItem _asbp_character_02_2)
          (goto _label))))))

(event EventBeginPlay
  (bind _z (Timeline|move_z Play)
    (:Update
      (Transformation|AddLocalOffset (Variables|Character|GetMesh) (Math|Vector|MakeVector 0.0 0.0 _z) false false))))

(event Collision|EventActorBeginOverlap
  (params (OtherActor :type Actor%20Object%20Reference)))

(event EventTick
  (params (DeltaSeconds :type Float%20%28single-precision%29))
  (Effects|SpawnEmitteratLocation "/Game/Goto/Whisp/WhispParticle.WhispParticle" (Transformation|GetWorldLocation (Variables|Character|GetMesh)) "0, 0, 0" "0.500000,0.500000,0.500000"))

(fn ConstructionScript)