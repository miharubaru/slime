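; BP_Wolf is an AI wolf that either of two local players can touch to score and collect as an item.
; Pawn sensing writes a seen BP_Character, the first player's class, into the blackboard's Player key.
; Mesh overlap with either character class calls that player's AddScoreWolf, sets ActorTrace, calls AddItem, then destroys the wolf.
; SetWolf repeats the first player's award with ActorTrace set to that character, without destroying the wolf.
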(event OnSeePawn(PawnSensing)
  (params (Pawn :type Pawn%20Object%20Reference))
  (bind _asbp_character (Utilities|Casting|CastToBP_Character Pawn))
  (AI|Components|Blackboard|SetValueasObject (AI|GetBlackboard self) (Utilities|Name|MakeLiteralName "Player") _asbp_character))

(event OnComponentBeginOverlap(StaticMesh)
  (params (OverlappedComponent :type Primitive%20Component%20Object%20Reference) (OtherActor :type Actor%20Object%20Reference) (OtherComp :type Primitive%20Component%20Object%20Reference) (OtherBodyIndex :type Integer) (bFromSweep :type Boolean) (SweepResult :type Hit%20Result%20Structure%20%28by%20ref%29))
  (bind _hitactor (Collision|BreakHitResult SweepResult))
  (Utilities|FlowControl|Sequence
    (:then_0
      (if (.bSuccess (Utilities|Casting|CastToBP_Character OtherActor))
        (CallFunction|WolfScoreBP01)
        (bind _asbp_character (Utilities|Casting|CastToBP_Character (Game|GetPlayerCharacter 0)))
        (Variables|/Game/BluePrints/BP_Character/BP_Character.BP_Character_C|SetActorTrace _asbp_character _hitactor)
        (Default|AddItem _asbp_character)
        (Actor|DestroyActor :!label _label)))
    (:then_1
      (if (.bSuccess (Utilities|Casting|CastToBP_Character_02 OtherActor))
        (CallFunction|WolfScoreBP02)
        (bind _asbp_character_02 (Utilities|Casting|CastToBP_Character_02 (Game|GetPlayerCharacter 1)))
        (Variables|/Game/BluePrints/BP_Character/BP_Character_02.BP_Character_02_C|SetActorTrace _asbp_character_02 _hitactor)
        (Default|AddItem _asbp_character_02)
        (goto _label)))))

(event EventTick
  (params (DeltaSeconds :type Float%20%28single-precision%29)))

(fn ConstructionScript)

(fn WolfScoreBP01
  (if true
    (bind _asbp_character (Utilities|Casting|CastToBP_Character (Game|Player|GetPlayerPawn 0)))
    (Default|AddScoreWolf _asbp_character)))

(fn WolfScoreBP02
  (if true
    (bind _asbp_character_02 (Utilities|Casting|CastToBP_Character_02 (Game|Player|GetPlayerPawn 1)))
    (Default|AddScoreWolf _asbp_character_02)))

(fn SetWolf
  (CallFunction|WolfScoreBP01)
  (bind _asbp_character (Utilities|Casting|CastToBP_Character (Game|GetPlayerCharacter 0)))
  (Variables|/Game/BluePrints/BP_Character/BP_Character.BP_Character_C|SetActorTrace _asbp_character _asbp_character)
  (Default|AddItem _asbp_character)
  (return))