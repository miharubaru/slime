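; Salamander enemy actor that grants the salamander ability to a player character who touches it with enough score.
; On box overlap, a sequence casts the other actor to each of four character Blueprints and compares its Score to its ScoreSalamander threshold.
; On a pass, it calls AbilityRisset and AddScoreSalamander, sets SalamanderAbility, then destroys itself.
; The same logic is duplicated per character class, with no shared parent cast or interface.
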(event OnComponentBeginOverlap(Box)
  (params (OverlappedComponent :type Primitive%20Component%20Object%20Reference) (OtherActor :type Actor%20Object%20Reference) (OtherComp :type Primitive%20Component%20Object%20Reference) (OtherBodyIndex :type Integer) (bFromSweep :type Boolean) (SweepResult :type Hit%20Result%20Structure%20%28by%20ref%29))
  (bind (_asbp_character _bsuccess) (Utilities|Casting|CastToBP_Character OtherActor))
  (bind (_asbp_character_02 _bsuccess_2) (Utilities|Casting|CastToBP_Character_02 OtherActor))
  (bind (_asbp_character_03 _bsuccess_3) (Utilities|Casting|CastToBP_Character_03 OtherActor))
  (bind (_asbp_character_04 _bsuccess_4) (Utilities|Casting|CastToBP_Character_04 OtherActor))
  (Utilities|FlowControl|Sequence
    (:then_0
      (if _bsuccess
        (if (>= (Variables|/Game/BluePrints/BP_Character/BP_Character.BP_Character_C|GetScore _asbp_character) (Variables|/Game/BluePrints/BP_Character/BP_Character.BP_Character_C|GetScoreSalamander _asbp_character))
          (Default|AbilityRisset _asbp_character)
          (Default|AddScoreSalamander _asbp_character)
          (Variables|/Game/BluePrints/BP_Character/BP_Character.BP_Character_C|SetSalamanderAbility _asbp_character true)
          (Actor|DestroyActor :!label _label))))
    (:then_1
      (if _bsuccess_2
        (if (>= (Variables|/Game/BluePrints/BP_Character/BP_Character_02.BP_Character_02_C|GetScore _asbp_character_02) (Variables|/Game/BluePrints/BP_Character/BP_Character_02.BP_Character_02_C|GetScoreSalamander _asbp_character_02))
          (Default|AbilityRisset _asbp_character_02)
          (Default|AddScoreSalamander _asbp_character_02)
          (Variables|/Game/BluePrints/BP_Character/BP_Character_02.BP_Character_02_C|SetSalamanderAbility _asbp_character_02 true)
          (goto _label))))
    (:then_2
      (if _bsuccess_3
        (if (>= (Variables|/Game/BluePrints/BP_Character/BP_Character_03.BP_Character_03_C|GetScore _asbp_character_03) (Variables|/Game/BluePrints/BP_Character/BP_Character_03.BP_Character_03_C|GetScoreSalamander _asbp_character_03))
          (Default|AbilityRisset _asbp_character_03)
          (Default|AddScoreSalamander _asbp_character_03)
          (Variables|/Game/BluePrints/BP_Character/BP_Character_03.BP_Character_03_C|SetSalamanderAbility _asbp_character_03 true)
          (goto _label))))
    (:then_3
      (if _bsuccess_4
        (if (>= (Variables|/Game/BluePrints/BP_Character/BP_Character_04.BP_Character_04_C|GetScore _asbp_character_04) (Variables|/Game/BluePrints/BP_Character/BP_Character_04.BP_Character_04_C|GetScoreSalamander _asbp_character_04))
          (Default|AbilityRisset _asbp_character_04)
          (Default|AddScoreSalamander _asbp_character_04)
          (Variables|/Game/BluePrints/BP_Character/BP_Character_04.BP_Character_04_C|SetSalamanderAbility _asbp_character_04 true)
          (goto _label))))))

(event EventBeginPlay)

(event Collision|EventActorBeginOverlap
  (params (OtherActor :type Actor%20Object%20Reference)))

(event EventTick
  (params (DeltaSeconds :type Float%20%28single-precision%29)))

(fn ConstructionScript)