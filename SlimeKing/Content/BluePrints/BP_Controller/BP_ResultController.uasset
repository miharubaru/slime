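; BP_ResultController is a controller Blueprint for the result screen, holding logic for a return-to-title Yes/No confirmation.
; Its graph checks GoTitle on BP_ResultMode, removes Title widgets, creates a YesNo widget and focuses its No button.
; A second branch uses GoTitle2 to show the existing dialog again.
; No event drives this chain, so it never runs as it stands, and the construction script is empty.
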(event Input|ActionEvents|InputActionClicke
  (params (Key :type Key%20Structure :default "None")))

(fn ConstructionScript)