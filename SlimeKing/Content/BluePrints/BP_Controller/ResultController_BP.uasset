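; ResultController_BP is a controller Blueprint for the result screen, holding logic for a return-to-title Yes/No prompt, but none of it is connected to an event.
; The disconnected chain reads GoTitle from ResultMode_BP, removes title widgets, then creates a prompt widget with focus on its No button.
; A second branch uses GoTitle2 to show that prompt again; debug prints remain and the construction script is empty.
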(event Input|ActionEvents|InputActionClicke
  (params (Key :type Key%20Structure)))

(fn ConstructionScript)