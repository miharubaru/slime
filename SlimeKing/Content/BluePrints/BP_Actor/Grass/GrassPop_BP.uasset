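; Level spawner that scatters grass, and bomb actors by their function names, at random points inside predefined bounds.
; BeginPlay spawns most grass zones at once, adds two large batches after long delays, and starts a timer counting GameTime down each second.
; When GameTime hits 61, Tick clears ExplosionBool and schedules a delayed bomb wave, plus a later one gated on that flag being true.
; GrassPop2 is never called.
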(event EventBeginPlay
  (Utilities|FlowControl|Sequence
    (:then_0
      (for _index (range 0 6)
        (CallFunction|GrassPop4)
        (CallFunction|GrassPop5)
        (CallFunction|GrassPop6)
        (CallFunction|GrassPop7)
        (CallFunction|GrassPop8)
        (CallFunction|GrassPop9)
        (CallFunction|GrassPop10)
        (CallFunction|GrassPop11)
        (CallFunction|GrassPop12)
        (CallFunction|GrassPop13)
        (CallFunction|GrassPop14)
        (CallFunction|GrassPop15)
        (CallFunction|GrassPop16)
        (CallFunction|GrassPop17)
        (CallFunction|GrassPop18)
        (CallFunction|GrassPop19)))
    (:then_1
      (for _index_2 (range 0 3)
        (CallFunction|GrassPop20)
        (CallFunction|GrassPop21)
        (CallFunction|GrassPop22)))
    (:then_2
      (Utilities|Time|SetTimerbyFunctionName 0 "GameTimeProgress" 1.0 true))
    (:then_3
      (Utilities|FlowControl|Sequence
        (:then_0
          (Utilities|FlowControl|Delay 7e+01)
          (for _index_3 (range 0 150)
            (CallFunction|GrassPop)))
        (:then_2
          (Utilities|FlowControl|Delay 1.5e+02)
          (for _index_4 (range 0 150)
            (CallFunction|GrassPop3)))))))

(event EventTick
  (params (DeltaSeconds :type Float%20%28single-precision%29))
  (if (== (Variables|Default|GetGameTime) 61)
    (Variables|Default|SetExplosionBool false)
    (Utilities|FlowControl|Sequence
      (:then_1
        (if (not (Variables|Default|GetExplosionBool))
          (Utilities|FlowControl|Delay 3e+01)
          (for _index (range 0 2)
            (CallFunction|BombPop)
            (CallFunction|BomPop2)
            (CallFunction|BombPop3)
            (CallFunction|BombPop4)
            (CallFunction|BombPop5)
            (CallFunction|BombPop6))))
      (:then_2
        (Utilities|FlowControl|Delay 7e+01)
        (if (Variables|Default|GetExplosionBool)
          (for _index_2 (range 0 2)
            (CallFunction|BombPop)
            (CallFunction|BomPop2)
            (CallFunction|BombPop3)
            (CallFunction|BombPop4)
            (CallFunction|BombPop5)
            (CallFunction|BombPop6)))))))

(fn ConstructionScript)

(fn GrassPop
  (bind _grass (Variables|Default|GetGrass))
  (bind _scale (Variables|Default|GetScale))
  (bind (_grass_2 _start _end _grass2 _grass3) (Utilities|Struct|BreakGrassPopStructure _grass))
  (bind (_x _y _z) (Math|Vector|BreakVector _end))
  (bind (_x_2 _y_2 _z_2) (Math|Vector|BreakVector _start))
  (bind _returnvalue (Math|Random|RandomFloatinRange _x_2 _x))
  (bind _returnvalue_2 (Math|Random|RandomFloatinRange _y_2 _y))
  (bind _returnvalue_3 (Math|Random|RandomFloatinRange _z_2 _z))
  (bind _returnvalue_4 (Math|Vector|MakeVector _returnvalue _returnvalue_2 _returnvalue_3))
  (bind _returnvalue_5 (Math|Transform|MakeTransform _returnvalue_4 "0,30.000000,0.000000" _scale))
  (Game|SpawnActorfromClass _grass_2 _returnvalue_5 "AlwaysSpawn" 0 0)
  (Game|SpawnActorfromClass _grass2 _returnvalue_5 "AlwaysSpawn" 0 0)
  (Game|SpawnActorfromClass _grass3 _returnvalue_5 "AlwaysSpawn" 0 0))

(fn GrassPop2
  (bind _grass2 (Variables|Default|GetGrass2))
  (bind _scale (Variables|Default|GetScale))
  (bind (_grass _start _end _grass2_2 _grass3) (Utilities|Struct|BreakGrassPopStructure _grass2))
  (bind (_x _y _z) (Math|Vector|BreakVector _end))
  (bind (_x_2 _y_2 _z_2) (Math|Vector|BreakVector _start))
  (bind _returnvalue (Math|Random|RandomFloatinRange _x_2 _x))
  (bind _returnvalue_2 (Math|Random|RandomFloatinRange _y_2 _y))
  (bind _returnvalue_3 (Math|Random|RandomFloatinRange _z_2 _z))
  (bind _returnvalue_4 (Math|Vector|MakeVector _returnvalue _returnvalue_2 _returnvalue_3))
  (bind _returnvalue_5 (Math|Transform|MakeTransform _returnvalue_4 "0,60.000000,0.000000" _scale))
  (Game|SpawnActorfromClass _grass _returnvalue_5 "AlwaysSpawn" 0 0)
  (Game|SpawnActorfromClass _grass2_2 _returnvalue_5 "AlwaysSpawn" 0 0)
  (Game|SpawnActorfromClass _grass3 _returnvalue_5 "AlwaysSpawn" 0 0))

(fn GrassPop3
  (bind _grass3 (Variables|Default|GetGrass3))
  (bind _scale (Variables|Default|GetScale))
  (bind (_grass _start _end _grass2 _grass3_2) (Utilities|Struct|BreakGrassPopStructure _grass3))
  (bind (_x _y _z) (Math|Vector|BreakVector _end))
  (bind (_x_2 _y_2 _z_2) (Math|Vector|BreakVector _start))
  (bind _returnvalue (Math|Random|RandomFloatinRange _x_2 _x))
  (bind _returnvalue_2 (Math|Random|RandomFloatinRange _y_2 _y))
  (bind _returnvalue_3 (Math|Random|RandomFloatinRange _z_2 _z))
  (bind _returnvalue_4 (Math|Vector|MakeVector _returnvalue _returnvalue_2 _returnvalue_3))
  (bind _returnvalue_5 (Math|Transform|MakeTransform _returnvalue_4 "0,90.000000,0.000000" _scale))
  (Game|SpawnActorfromClass _grass _returnvalue_5 "AlwaysSpawn" 0 0)
  (Game|SpawnActorfromClass _grass2 _returnvalue_5 "AlwaysSpawn" 0 0)
  (Game|SpawnActorfromClass _grass3_2 _returnvalue_5 "AlwaysSpawn" 0 0))

(fn GrassPop4
  (bind _grass4 (Variables|Default|GetGrass4))
  (bind _scale (Variables|Default|GetScale))
  (bind (_grass _start _end _grass2 _grass3) (Utilities|Struct|BreakGrassPopStructure _grass4))
  (bind (_x _y _z) (Math|Vector|BreakVector _end))
  (bind (_x_2 _y_2 _z_2) (Math|Vector|BreakVector _start))
  (bind _returnvalue (Math|Random|RandomFloatinRange _x_2 _x))
  (bind _returnvalue_2 (Math|Random|RandomFloatinRange _y_2 _y))
  (bind _returnvalue_3 (Math|Random|RandomFloatinRange _z_2 _z))
  (bind _returnvalue_4 (Math|Vector|MakeVector _returnvalue _returnvalue_2 _returnvalue_3))
  (bind _returnvalue_5 (Math|Transform|MakeTransform _returnvalue_4 "0,120.000000,0.000000" _scale))
  (Game|SpawnActorfromClass _grass _returnvalue_5 "AlwaysSpawn" 0 0)
  (Game|SpawnActorfromClass _grass2 _returnvalue_5 "AlwaysSpawn" 0 0)
  (Game|SpawnActorfromClass _grass3 _returnvalue_5 "AlwaysSpawn" 0 0))

(fn GrassPop5
  (bind _scale (Variables|Default|GetScale))
  (bind _grass5 (Variables|Default|GetGrass5))
  (bind (_grass _start _end _grass2 _grass3) (Utilities|Struct|BreakGrassPopStructure _grass5))
  (bind (_x _y _z) (Math|Vector|BreakVector _end))
  (bind (_x_2 _y_2 _z_2) (Math|Vector|BreakVector _start))
  (bind _returnvalue (Math|Random|RandomFloatinRange _x_2 _x))
  (bind _returnvalue_2 (Math|Random|RandomFloatinRange _y_2 _y))
  (bind _returnvalue_3 (Math|Random|RandomFloatinRange _z_2 _z))
  (bind _returnvalue_4 (Math|Vector|MakeVector _returnvalue _returnvalue_2 _returnvalue_3))
  (bind _returnvalue_5 (Math|Transform|MakeTransform _returnvalue_4 "0,150.000000,0.000000" _scale))
  (Game|SpawnActorfromClass _grass _returnvalue_5 "AlwaysSpawn" 0 0)
  (Game|SpawnActorfromClass _grass2 _returnvalue_5 "AlwaysSpawn" 0 0)
  (Game|SpawnActorfromClass _grass3 _returnvalue_5 "AlwaysSpawn" 0 0))

(fn GrassPop6
  (bind _scale (Variables|Default|GetScale))
  (bind _grass6 (Variables|Default|GetGrass6))
  (bind (_grass _start _end _grass2 _grass3) (Utilities|Struct|BreakGrassPopStructure _grass6))
  (bind (_x _y _z) (Math|Vector|BreakVector _end))
  (bind (_x_2 _y_2 _z_2) (Math|Vector|BreakVector _start))
  (bind _returnvalue (Math|Random|RandomFloatinRange _x_2 _x))
  (bind _returnvalue_2 (Math|Random|RandomFloatinRange _y_2 _y))
  (bind _returnvalue_3 (Math|Random|RandomFloatinRange _z_2 _z))
  (bind _returnvalue_4 (Math|Vector|MakeVector _returnvalue _returnvalue_2 _returnvalue_3))
  (bind _returnvalue_5 (Math|Transform|MakeTransform _returnvalue_4 "0,180.000000,0.000000" _scale))
  (Game|SpawnActorfromClass _grass _returnvalue_5 "AlwaysSpawn" 0 0)
  (Game|SpawnActorfromClass _grass2 _returnvalue_5 "AlwaysSpawn" 0 0)
  (Game|SpawnActorfromClass _grass3 _returnvalue_5 "AlwaysSpawn" 0 0))

(fn GrassPop7
  (bind _scale (Variables|Default|GetScale))
  (bind _grass7 (Variables|Default|GetGrass7))
  (bind (_grass _start _end _grass2 _grass3) (Utilities|Struct|BreakGrassPopStructure _grass7))
  (bind (_x _y _z) (Math|Vector|BreakVector _end))
  (bind (_x_2 _y_2 _z_2) (Math|Vector|BreakVector _start))
  (bind _returnvalue (Math|Random|RandomFloatinRange _x_2 _x))
  (bind _returnvalue_2 (Math|Random|RandomFloatinRange _y_2 _y))
  (bind _returnvalue_3 (Math|Random|RandomFloatinRange _z_2 _z))
  (bind _returnvalue_4 (Math|Vector|MakeVector _returnvalue _returnvalue_2 _returnvalue_3))
  (bind _returnvalue_5 (Math|Transform|MakeTransform _returnvalue_4 "0,50.000000,0.000000" _scale))
  (Game|SpawnActorfromClass _grass _returnvalue_5 "AlwaysSpawn" 0 0)
  (Game|SpawnActorfromClass _grass2 _returnvalue_5 "AlwaysSpawn" 0 0)
  (Game|SpawnActorfromClass _grass3 _returnvalue_5 "AlwaysSpawn" 0 0))

(fn GrassPop8
  (bind _scale (Variables|Default|GetScale))
  (bind _grass8 (Variables|Default|GetGrass8))
  (bind (_grass _start _end _grass2 _grass3) (Utilities|Struct|BreakGrassPopStructure _grass8))
  (bind (_x _y _z) (Math|Vector|BreakVector _end))
  (bind (_x_2 _y_2 _z_2) (Math|Vector|BreakVector _start))
  (bind _returnvalue (Math|Random|RandomFloatinRange _x_2 _x))
  (bind _returnvalue_2 (Math|Random|RandomFloatinRange _y_2 _y))
  (bind _returnvalue_3 (Math|Random|RandomFloatinRange _z_2 _z))
  (bind _returnvalue_4 (Math|Vector|MakeVector _returnvalue _returnvalue_2 _returnvalue_3))
  (bind _returnvalue_5 (Math|Transform|MakeTransform _returnvalue_4 "0,100.000000,0.000000" _scale))
  (Game|SpawnActorfromClass _grass _returnvalue_5 "AlwaysSpawn" 0 0)
  (Game|SpawnActorfromClass _grass2 _returnvalue_5 "AlwaysSpawn" 0 0)
  (Game|SpawnActorfromClass _grass3 _returnvalue_5 "AlwaysSpawn" 0 0))

(fn GrassPop9
  (bind _scale (Variables|Default|GetScale))
  (bind _grass9 (Variables|Default|GetGrass9))
  (bind (_grass _start _end _grass2 _grass3) (Utilities|Struct|BreakGrassPopStructure _grass9))
  (bind (_x _y _z) (Math|Vector|BreakVector _end))
  (bind (_x_2 _y_2 _z_2) (Math|Vector|BreakVector _start))
  (bind _returnvalue (Math|Random|RandomFloatinRange _x_2 _x))
  (bind _returnvalue_2 (Math|Random|RandomFloatinRange _y_2 _y))
  (bind _returnvalue_3 (Math|Random|RandomFloatinRange _z_2 _z))
  (bind _returnvalue_4 (Math|Vector|MakeVector _returnvalue _returnvalue_2 _returnvalue_3))
  (bind _returnvalue_5 (Math|Transform|MakeTransform _returnvalue_4 "0,150.000000,0.000000" _scale))
  (Game|SpawnActorfromClass _grass _returnvalue_5 "AlwaysSpawn" 0 0)
  (Game|SpawnActorfromClass _grass2 _returnvalue_5 "AlwaysSpawn" 0 0)
  (Game|SpawnActorfromClass _grass3 _returnvalue_5 "AlwaysSpawn" 0 0))

(fn GrassPop10
  (bind _scale (Variables|Default|GetScale))
  (bind _grass10 (Variables|Default|GetGrass10))
  (bind (_grass _start _end _grass2 _grass3) (Utilities|Struct|BreakGrassPopStructure _grass10))
  (bind (_x _y _z) (Math|Vector|BreakVector _end))
  (bind (_x_2 _y_2 _z_2) (Math|Vector|BreakVector _start))
  (bind _returnvalue (Math|Random|RandomFloatinRange _x_2 _x))
  (bind _returnvalue_2 (Math|Random|RandomFloatinRange _y_2 _y))
  (bind _returnvalue_3 (Math|Random|RandomFloatinRange _z_2 _z))
  (bind _returnvalue_4 (Math|Vector|MakeVector _returnvalue _returnvalue_2 _returnvalue_3))
  (bind _returnvalue_5 (Math|Transform|MakeTransform _returnvalue_4 "0,200.000000, 0" _scale))
  (Game|SpawnActorfromClass _grass _returnvalue_5 "AlwaysSpawn" 0 0)
  (Game|SpawnActorfromClass _grass2 _returnvalue_5 "AlwaysSpawn" 0 0)
  (Game|SpawnActorfromClass _grass3 _returnvalue_5 "AlwaysSpawn" 0 0))

(fn GrassPop11
  (bind _scale (Variables|Default|GetScale))
  (bind _grass11 (Variables|Default|GetGrass11))
  (bind (_grass _start _end _grass2 _grass3) (Utilities|Struct|BreakGrassPopStructure _grass11))
  (bind (_x _y _z) (Math|Vector|BreakVector _end))
  (bind (_x_2 _y_2 _z_2) (Math|Vector|BreakVector _start))
  (bind _returnvalue (Math|Random|RandomFloatinRange _x_2 _x))
  (bind _returnvalue_2 (Math|Random|RandomFloatinRange _y_2 _y))
  (bind _returnvalue_3 (Math|Random|RandomFloatinRange _z_2 _z))
  (bind _returnvalue_4 (Math|Vector|MakeVector _returnvalue _returnvalue_2 _returnvalue_3))
  (bind _returnvalue_5 (Math|Transform|MakeTransform _returnvalue_4 "0,250.000000, 0" _scale))
  (Game|SpawnActorfromClass _grass _returnvalue_5 "AlwaysSpawn" 0 0)
  (Game|SpawnActorfromClass _grass2 _returnvalue_5 "AlwaysSpawn" 0 0)
  (Game|SpawnActorfromClass _grass3 _returnvalue_5 "AlwaysSpawn" 0 0))

(fn GrassPop12
  (bind _grass12 (Variables|Default|GetGrass12))
  (bind _scale (Variables|Default|GetScale))
  (bind (_grass _start _end _grass2 _grass3) (Utilities|Struct|BreakGrassPopStructure _grass12))
  (bind (_x _y _z) (Math|Vector|BreakVector _end))
  (bind (_x_2 _y_2 _z_2) (Math|Vector|BreakVector _start))
  (bind _returnvalue (Math|Random|RandomFloatinRange _x_2 _x))
  (bind _returnvalue_2 (Math|Random|RandomFloatinRange _y_2 _y))
  (bind _returnvalue_3 (Math|Random|RandomFloatinRange _z_2 _z))
  (bind _returnvalue_4 (Math|Vector|MakeVector _returnvalue _returnvalue_2 _returnvalue_3))
  (bind _returnvalue_5 (Math|Transform|MakeTransform _returnvalue_4 "0,300.000000, 0" _scale))
  (Game|SpawnActorfromClass _grass _returnvalue_5 "AlwaysSpawn" 0 0)
  (Game|SpawnActorfromClass _grass2 _returnvalue_5 "AlwaysSpawn" 0 0)
  (Game|SpawnActorfromClass _grass3 _returnvalue_5 "AlwaysSpawn" 0 0))

(fn GrassPop13
  (bind _grass13 (Variables|Default|GetGrass13))
  (bind _scale (Variables|Default|GetScale))
  (bind (_grass _start _end _grass2 _grass3) (Utilities|Struct|BreakGrassPopStructure _grass13))
  (bind (_x _y _z) (Math|Vector|BreakVector _end))
  (bind (_x_2 _y_2 _z_2) (Math|Vector|BreakVector _start))
  (bind _returnvalue (Math|Random|RandomFloatinRange _x_2 _x))
  (bind _returnvalue_2 (Math|Random|RandomFloatinRange _y_2 _y))
  (bind _returnvalue_3 (Math|Random|RandomFloatinRange _z_2 _z))
  (bind _returnvalue_4 (Math|Vector|MakeVector _returnvalue _returnvalue_2 _returnvalue_3))
  (bind _returnvalue_5 (Math|Transform|MakeTransform _returnvalue_4 "0,350.000000, 0" _scale))
  (Game|SpawnActorfromClass _grass _returnvalue_5 "AlwaysSpawn" 0 0)
  (Game|SpawnActorfromClass _grass2 _returnvalue_5 "AlwaysSpawn" 0 0)
  (Game|SpawnActorfromClass _grass3 _returnvalue_5 "AlwaysSpawn" 0 0))

(fn GrassPop14
  (bind _grass14 (Variables|Default|GetGrass14))
  (bind _scale (Variables|Default|GetScale))
  (bind (_grass _start _end _grass2 _grass3) (Utilities|Struct|BreakGrassPopStructure _grass14))
  (bind (_x _y _z) (Math|Vector|BreakVector _end))
  (bind (_x_2 _y_2 _z_2) (Math|Vector|BreakVector _start))
  (bind _returnvalue (Math|Random|RandomFloatinRange _x_2 _x))
  (bind _returnvalue_2 (Math|Random|RandomFloatinRange _y_2 _y))
  (bind _returnvalue_3 (Math|Random|RandomFloatinRange _z_2 _z))
  (bind _returnvalue_4 (Math|Vector|MakeVector _returnvalue _returnvalue_2 _returnvalue_3))
  (bind _returnvalue_5 (Math|Transform|MakeTransform _returnvalue_4 "0,40.000000, 0" _scale))
  (Game|SpawnActorfromClass _grass _returnvalue_5 "AlwaysSpawn" 0 0)
  (Game|SpawnActorfromClass _grass2 _returnvalue_5 "AlwaysSpawn" 0 0)
  (Game|SpawnActorfromClass _grass3 _returnvalue_5 "AlwaysSpawn" 0 0))

(fn GrassPop15
  (bind _grass15 (Variables|Default|GetGrass15))
  (bind _scale (Variables|Default|GetScale))
  (bind (_grass _start _end _grass2 _grass3) (Utilities|Struct|BreakGrassPopStructure _grass15))
  (bind (_x _y _z) (Math|Vector|BreakVector _end))
  (bind (_x_2 _y_2 _z_2) (Math|Vector|BreakVector _start))
  (bind _returnvalue (Math|Random|RandomFloatinRange _x_2 _x))
  (bind _returnvalue_2 (Math|Random|RandomFloatinRange _y_2 _y))
  (bind _returnvalue_3 (Math|Random|RandomFloatinRange _z_2 _z))
  (bind _returnvalue_4 (Math|Vector|MakeVector _returnvalue _returnvalue_2 _returnvalue_3))
  (bind _returnvalue_5 (Math|Transform|MakeTransform _returnvalue_4 "0,80.000000, 0" _scale))
  (Game|SpawnActorfromClass _grass _returnvalue_5 "AlwaysSpawn" 0 0)
  (Game|SpawnActorfromClass _grass2 _returnvalue_5 "AlwaysSpawn" 0 0)
  (Game|SpawnActorfromClass _grass3 _returnvalue_5 "AlwaysSpawn" 0 0))

(fn GrassPop16
  (bind _grass16 (Variables|Default|GetGrass16))
  (bind _scale (Variables|Default|GetScale))
  (bind (_grass _start _end _grass2 _grass3) (Utilities|Struct|BreakGrassPopStructure _grass16))
  (bind (_x _y _z) (Math|Vector|BreakVector _end))
  (bind (_x_2 _y_2 _z_2) (Math|Vector|BreakVector _start))
  (bind _returnvalue (Math|Random|RandomFloatinRange _x_2 _x))
  (bind _returnvalue_2 (Math|Random|RandomFloatinRange _y_2 _y))
  (bind _returnvalue_3 (Math|Random|RandomFloatinRange _z_2 _z))
  (bind _returnvalue_4 (Math|Vector|MakeVector _returnvalue _returnvalue_2 _returnvalue_3))
  (bind _returnvalue_5 (Math|Transform|MakeTransform _returnvalue_4 "0,120.000000, 0" _scale))
  (Game|SpawnActorfromClass _grass _returnvalue_5 "AlwaysSpawn" 0 0)
  (Game|SpawnActorfromClass _grass2 _returnvalue_5 "AlwaysSpawn" 0 0)
  (Game|SpawnActorfromClass _grass3 _returnvalue_5 "AlwaysSpawn" 0 0))

(fn GrassPop17
  (bind _grass17 (Variables|Default|GetGrass17))
  (bind _scale (Variables|Default|GetScale))
  (bind (_grass _start _end _grass2 _grass3) (Utilities|Struct|BreakGrassPopStructure _grass17))
  (bind (_x _y _z) (Math|Vector|BreakVector _end))
  (bind (_x_2 _y_2 _z_2) (Math|Vector|BreakVector _start))
  (bind _returnvalue (Math|Random|RandomFloatinRange _x_2 _x))
  (bind _returnvalue_2 (Math|Random|RandomFloatinRange _y_2 _y))
  (bind _returnvalue_3 (Math|Random|RandomFloatinRange _z_2 _z))
  (bind _returnvalue_4 (Math|Vector|MakeVector _returnvalue _returnvalue_2 _returnvalue_3))
  (bind _returnvalue_5 (Math|Transform|MakeTransform _returnvalue_4 "0,160.000000, 0" _scale))
  (Game|SpawnActorfromClass _grass _returnvalue_5 "AlwaysSpawn" 0 0)
  (Game|SpawnActorfromClass _grass2 _returnvalue_5 "AlwaysSpawn" 0 0)
  (Game|SpawnActorfromClass _grass3 _returnvalue_5 "AlwaysSpawn" 0 0))

(fn GrassPop18
  (bind _grass18 (Variables|Default|GetGrass18))
  (bind _scale (Variables|Default|GetScale))
  (bind (_grass _start _end _grass2 _grass3) (Utilities|Struct|BreakGrassPopStructure _grass18))
  (bind (_x _y _z) (Math|Vector|BreakVector _end))
  (bind (_x_2 _y_2 _z_2) (Math|Vector|BreakVector _start))
  (bind _returnvalue (Math|Random|RandomFloatinRange _x_2 _x))
  (bind _returnvalue_2 (Math|Random|RandomFloatinRange _y_2 _y))
  (bind _returnvalue_3 (Math|Random|RandomFloatinRange _z_2 _z))
  (bind _returnvalue_4 (Math|Vector|MakeVector _returnvalue _returnvalue_2 _returnvalue_3))
  (bind _returnvalue_5 (Math|Transform|MakeTransform _returnvalue_4 "0,200.000000, 0" _scale))
  (Game|SpawnActorfromClass _grass _returnvalue_5 "AlwaysSpawn" 0 0)
  (Game|SpawnActorfromClass _grass2 _returnvalue_5 "AlwaysSpawn" 0 0)
  (Game|SpawnActorfromClass _grass3 _returnvalue_5 "AlwaysSpawn" 0 0))

(fn GrassPop19
  (bind _grass19 (Variables|Default|GetGrass19))
  (bind _scale (Variables|Default|GetScale))
  (bind (_grass _start _end _grass2 _grass3) (Utilities|Struct|BreakGrassPopStructure _grass19))
  (bind (_x _y _z) (Math|Vector|BreakVector _end))
  (bind (_x_2 _y_2 _z_2) (Math|Vector|BreakVector _start))
  (bind _returnvalue (Math|Random|RandomFloatinRange _x_2 _x))
  (bind _returnvalue_2 (Math|Random|RandomFloatinRange _y_2 _y))
  (bind _returnvalue_3 (Math|Random|RandomFloatinRange _z_2 _z))
  (bind _returnvalue_4 (Math|Vector|MakeVector _returnvalue _returnvalue_2 _returnvalue_3))
  (bind _returnvalue_5 (Math|Transform|MakeTransform _returnvalue_4 "0,240.000000, 0" _scale))
  (Game|SpawnActorfromClass _grass _returnvalue_5 "AlwaysSpawn" 0 0)
  (Game|SpawnActorfromClass _grass2 _returnvalue_5 "AlwaysSpawn" 0 0)
  (Game|SpawnActorfromClass _grass3 _returnvalue_5 "AlwaysSpawn" 0 0))

(fn GrassPop20
  (bind _grass20 (Variables|Default|GetGrass20))
  (bind _scale (Variables|Default|GetScale))
  (bind (_grass _start _end _grass2 _grass3) (Utilities|Struct|BreakGrassPopStructure _grass20))
  (bind (_x _y _z) (Math|Vector|BreakVector _end))
  (bind (_x_2 _y_2 _z_2) (Math|Vector|BreakVector _start))
  (bind _returnvalue (Math|Random|RandomFloatinRange _x_2 _x))
  (bind _returnvalue_2 (Math|Random|RandomFloatinRange _y_2 _y))
  (bind _returnvalue_3 (Math|Random|RandomFloatinRange _z_2 _z))
  (bind _returnvalue_4 (Math|Vector|MakeVector _returnvalue _returnvalue_2 _returnvalue_3))
  (bind _returnvalue_5 (Math|Transform|MakeTransform _returnvalue_4 "0,280.000000, 0" _scale))
  (Game|SpawnActorfromClass _grass _returnvalue_5 "AlwaysSpawn" 0 0)
  (Game|SpawnActorfromClass _grass2 _returnvalue_5 "AlwaysSpawn" 0 0)
  (Game|SpawnActorfromClass _grass3 _returnvalue_5 "AlwaysSpawn" 0 0))

(fn GrassPop21
  (bind _grass21 (Variables|Default|GetGrass21))
  (bind _scale (Variables|Default|GetScale))
  (bind (_grass _start _end _grass2 _grass3) (Utilities|Struct|BreakGrassPopStructure _grass21))
  (bind (_x _y _z) (Math|Vector|BreakVector _end))
  (bind (_x_2 _y_2 _z_2) (Math|Vector|BreakVector _start))
  (bind _returnvalue (Math|Random|RandomFloatinRange _x_2 _x))
  (bind _returnvalue_2 (Math|Random|RandomFloatinRange _y_2 _y))
  (bind _returnvalue_3 (Math|Random|RandomFloatinRange _z_2 _z))
  (bind _returnvalue_4 (Math|Vector|MakeVector _returnvalue _returnvalue_2 _returnvalue_3))
  (bind _returnvalue_5 (Math|Transform|MakeTransform _returnvalue_4 "0,320.000000, 0" _scale))
  (Game|SpawnActorfromClass _grass _returnvalue_5 "AlwaysSpawn" 0 0)
  (Game|SpawnActorfromClass _grass2 _returnvalue_5 "AlwaysSpawn" 0 0)
  (Game|SpawnActorfromClass _grass3 _returnvalue_5 "AlwaysSpawn" 0 0))

(fn BombPop
  (bind _ex (Variables|Default|GetEx))
  (bind (_grass _start _end) (Utilities|Struct|BreakGrassPopStructure _ex))
  (bind (_x _y _z) (Math|Vector|BreakVector _end))
  (bind (_x_2 _y_2 _z_2) (Math|Vector|BreakVector _start))
  (Game|SpawnActorfromClass _grass (Math|Transform|MakeTransform (Math|Vector|MakeVector (Math|Random|RandomFloatinRange _x_2 _x) (Math|Random|RandomFloatinRange _y_2 _y) (Math|Random|RandomFloatinRange _z_2 _z)) "0,20.000000, 0") "AlwaysSpawn" 0 0))

(fn BomPop2
  (bind _ex2 (Variables|Default|GetEx2))
  (bind (_grass _start _end) (Utilities|Struct|BreakGrassPopStructure _ex2))
  (bind (_x _y _z) (Math|Vector|BreakVector _end))
  (bind (_x_2 _y_2 _z_2) (Math|Vector|BreakVector _start))
  (Game|SpawnActorfromClass _grass (Math|Transform|MakeTransform (Math|Vector|MakeVector (Math|Random|RandomFloatinRange _x_2 _x) (Math|Random|RandomFloatinRange _y_2 _y) (Math|Random|RandomFloatinRange _z_2 _z)) "0,40.000000, 0") "AlwaysSpawn" 0 0))

(fn BombPop3
  (bind _ex3 (Variables|Default|GetEx3))
  (bind (_grass _start _end _grass2 _grass3) (Utilities|Struct|BreakGrassPopStructure _ex3))
  (bind (_x _y _z) (Math|Vector|BreakVector _end))
  (bind (_x_2 _y_2 _z_2) (Math|Vector|BreakVector _start))
  (bind _returnvalue (Math|Random|RandomFloatinRange _x_2 _x))
  (bind _returnvalue_2 (Math|Random|RandomFloatinRange _y_2 _y))
  (bind _returnvalue_3 (Math|Random|RandomFloatinRange _z_2 _z))
  (bind _returnvalue_4 (Math|Vector|MakeVector _returnvalue _returnvalue_2 _returnvalue_3))
  (bind _returnvalue_5 (Math|Transform|MakeTransform _returnvalue_4 "0,70.000000, 0"))
  (Game|SpawnActorfromClass _grass _returnvalue_5 "AlwaysSpawn" 0 0)
  (Game|SpawnActorfromClass _grass2 _returnvalue_5 "AlwaysSpawn" 0 0)
  (Game|SpawnActorfromClass _grass3 _returnvalue_5 "AlwaysSpawn" 0 0))

(fn BombPop4
  (bind _ex4 (Variables|Default|GetEx4))
  (bind (_grass _start _end _grass2 _grass3) (Utilities|Struct|BreakGrassPopStructure _ex4))
  (bind (_x _y _z) (Math|Vector|BreakVector _end))
  (bind (_x_2 _y_2 _z_2) (Math|Vector|BreakVector _start))
  (bind _returnvalue (Math|Random|RandomFloatinRange _x_2 _x))
  (bind _returnvalue_2 (Math|Random|RandomFloatinRange _y_2 _y))
  (bind _returnvalue_3 (Math|Random|RandomFloatinRange _z_2 _z))
  (bind _returnvalue_4 (Math|Vector|MakeVector _returnvalue _returnvalue_2 _returnvalue_3))
  (bind _returnvalue_5 (Math|Transform|MakeTransform _returnvalue_4 "0,90.000000, 0"))
  (Game|SpawnActorfromClass _grass _returnvalue_5 "AlwaysSpawn" 0 0)
  (Game|SpawnActorfromClass _grass2 _returnvalue_5 "AlwaysSpawn" 0 0)
  (Game|SpawnActorfromClass _grass3 _returnvalue_5 "AlwaysSpawn" 0 0))

(fn BombPop5
  (bind _ex5 (Variables|Default|GetEx5))
  (bind (_grass _start _end _grass2 _grass3) (Utilities|Struct|BreakGrassPopStructure _ex5))
  (bind (_x _y _z) (Math|Vector|BreakVector _end))
  (bind (_x_2 _y_2 _z_2) (Math|Vector|BreakVector _start))
  (bind _returnvalue (Math|Random|RandomFloatinRange _x_2 _x))
  (bind _returnvalue_2 (Math|Random|RandomFloatinRange _y_2 _y))
  (bind _returnvalue_3 (Math|Random|RandomFloatinRange _z_2 _z))
  (bind _returnvalue_4 (Math|Vector|MakeVector _returnvalue _returnvalue_2 _returnvalue_3))
  (bind _returnvalue_5 (Math|Transform|MakeTransform _returnvalue_4 "0,130.000000, 0"))
  (Game|SpawnActorfromClass _grass _returnvalue_5 "AlwaysSpawn" 0 0)
  (Game|SpawnActorfromClass _grass2 _returnvalue_5 "AlwaysSpawn" 0 0)
  (Game|SpawnActorfromClass _grass3 _returnvalue_5 "AlwaysSpawn" 0 0))

(fn BombPop6
  (bind _ex6 (Variables|Default|GetEx6))
  (bind (_grass _start _end _grass2 _grass3) (Utilities|Struct|BreakGrassPopStructure _ex6))
  (bind (_x _y _z) (Math|Vector|BreakVector _end))
  (bind (_x_2 _y_2 _z_2) (Math|Vector|BreakVector _start))
  (bind _returnvalue (Math|Random|RandomFloatinRange _x_2 _x))
  (bind _returnvalue_2 (Math|Random|RandomFloatinRange _y_2 _y))
  (bind _returnvalue_3 (Math|Random|RandomFloatinRange _z_2 _z))
  (bind _returnvalue_4 (Math|Vector|MakeVector _returnvalue _returnvalue_2 _returnvalue_3))
  (bind _returnvalue_5 (Math|Transform|MakeTransform _returnvalue_4 "0,150.000000, 0"))
  (Game|SpawnActorfromClass _grass _returnvalue_5 "AlwaysSpawn" 0 0)
  (Game|SpawnActorfromClass _grass2 _returnvalue_5 "AlwaysSpawn" 0 0)
  (Game|SpawnActorfromClass _grass3 _returnvalue_5 "AlwaysSpawn" 0 0))

(fn GrassPop22
  (bind _scale (Variables|Default|GetScale))
  (bind _grass22 (Variables|Default|GetGrass22))
  (bind (_grass _start _end _grass2 _grass3) (Utilities|Struct|BreakGrassPopStructure _grass22))
  (bind (_x _y _z) (Math|Vector|BreakVector _end))
  (bind (_x_2 _y_2 _z_2) (Math|Vector|BreakVector _start))
  (bind _returnvalue (Math|Random|RandomFloatinRange _x_2 _x))
  (bind _returnvalue_2 (Math|Random|RandomFloatinRange _y_2 _y))
  (bind _returnvalue_3 (Math|Random|RandomFloatinRange _z_2 _z))
  (bind _returnvalue_4 (Math|Vector|MakeVector _returnvalue _returnvalue_2 _returnvalue_3))
  (bind _returnvalue_5 (Math|Transform|MakeTransform _returnvalue_4 "0,320.000000, 0" _scale))
  (Game|SpawnActorfromClass _grass _returnvalue_5 "AlwaysSpawn" 0 0)
  (Game|SpawnActorfromClass _grass2 _returnvalue_5 "AlwaysSpawn" 0 0)
  (Game|SpawnActorfromClass _grass3 _returnvalue_5 "AlwaysSpawn" 0 0))

(fn GameTimeProgress
  (if (> (Variables|Default|GetGameTime) 0)
    (bind _result (Math|Integer|DecrementInt (Variables|Default|GetGameTime))
      (:%20%20
        (Variables|Default|SetGameTime _result)
        (return)))))