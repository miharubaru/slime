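; MombGrass_BP is a grass pickup that grants the explosion ability to whichever of four player character classes touches it.
; On StaticMesh overlap it casts the other actor to each character class in sequence.
; A match resets that character's abilities, adds score, sets its explosion flag, plays the acquired sound at the GameInstace_BP volume, then destroys the pickup.
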(event OnComponentBeginOverlap(StaticMesh)
  (params (OverlappedComponent :type Primitive%20Component%20Object%20Reference) (OtherActor :type Actor%20Object%20Reference) (OtherComp :type Primitive%20Component%20Object%20Reference) (OtherBodyIndex :type Integer) (bFromSweep :type Boolean) (SweepResult :type Hit%20Result%20Structure%20%28by%20ref%29))
  (bind (_asbp_character _bsuccess) (Utilities|Casting|CastToBP_Character OtherActor))
  (bind (_asbp_character_02 _bsuccess_2) (Utilities|Casting|CastToBP_Character_02 OtherActor))
  (bind (_asbp_character_03 _bsuccess_3) (Utilities|Casting|CastToBP_Character_03 OtherActor))
  (bind (_asbp_character_04 _bsuccess_4) (Utilities|Casting|CastToBP_Character_04 OtherActor))
  (bind _asgame_instace_bp (Utilities|Casting|CastToGameInstace_BP (Game|GetGameInstance)))
  (Variables|Default|SetAbilityAcquiredVolume (Variables|/Game/BluePrints/BP_Instance/GameInstace_BP.GameInstace_BP_C|GetAbilityAcquiredVolume _asgame_instace_bp))
  (Utilities|FlowControl|Sequence
    (:then_0
      (if _bsuccess
        (Default|AbilityRisset _asbp_character)
        (Default|AddScore _asbp_character)
        (Audio|PlaySound2D "/Game/Sounds/22_Slime_AvilityAcquired.22_Slime_AvilityAcquired" (Variables|Default|GetAbilityAcquiredVolume) 1.0 0.0 0 0)
        (Variables|/Game/BluePrints/BP_Character/BP_Character.BP_Character_C|SetExplosionAbility _asbp_character true)
        (Actor|DestroyActor :!label _label)))
    (:then_1
      (if _bsuccess_2
        (Default|AbilityRisset _asbp_character_02)
        (Default|AddScore _asbp_character_02)
        (Audio|PlaySound2D "/Game/Sounds/22_Slime_AvilityAcquired.22_Slime_AvilityAcquired" (Variables|Default|GetAbilityAcquiredVolume) 1.0 0.0 0 0)
        (Variables|/Game/BluePrints/BP_Character/BP_Character_02.BP_Character_02_C|SetExplosiopnAbility _asbp_character_02 true)
        (goto _label)))
    (:then_2
      (if _bsuccess_3
        (Default|AbilityRisset _asbp_character_03)
        (Default|AddScore _asbp_character_03)
        (Audio|PlaySound2D "/Game/Sounds/22_Slime_AvilityAcquired.22_Slime_AvilityAcquired" (Variables|Default|GetAbilityAcquiredVolume) 1.0 0.0 0 0)
        (Variables|/Game/BluePrints/BP_Character/BP_Character_03.BP_Character_03_C|SetExplosionAbility _asbp_character_03 true)
        (goto _label)))
    (:then_3
      (if _bsuccess_4
        (Default|AbilityRisset _asbp_character_04)
        (Default|AddScore _asbp_character_04)
        (Audio|PlaySound2D "/Game/Sounds/22_Slime_AvilityAcquired.22_Slime_AvilityAcquired" (Variables|Default|GetAbilityAcquiredVolume) 1.0 0.0 0 0)
        (Variables|/Game/BluePrints/BP_Character/BP_Character_04.BP_Character_04_C|SetExplosionAbility _asbp_character_04 true)
        (goto _label)))))

(event EventBeginPlay)

(event Collision|EventActorBeginOverlap
  (params (OtherActor :type Actor%20Object%20Reference)))

(event EventTick
  (params (DeltaSeconds :type Float%20%28single-precision%29)))

(fn ConstructionScript
  (|CallParentFunction))