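; Timed event actor that spawns a Salamander with its default controller once a countdown reaches zero.
; A looping one-second timer decrements GameTime, and Tick watches for zero, using a flag to run the fixed-transform spawn only once.
; Separate helpers spawn Wolf, Wisp, winged Rabbit and Lizard enemies at random points within per-type areas, but nothing in this Blueprint calls them.
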(event EventBeginPlay
  (Utilities|Time|SetTimerbyFunctionName 0 "SetTime" 1.0 true))

(event EventTick
  (params (DeltaSeconds :type Float%20%28single-precision%29))
  (if (== (Variables|Default|GetGameTime) 0)
    (if (not (Variables|Default|GetEvent?))
      (CallFunction|SetSpawn)
      (Variables|Default|SetEvent? true))))

(fn ConstructionScript)

(fn SetTime
  (if (> (Variables|Default|GetGameTime) 0)
    (bind _result (Math|Integer|DecrementInt (Variables|Default|GetGameTime))
      (:%20%20
        (Variables|Default|SetGameTime _result)))))

(fn SetWolf
  (bind _wolf (Variables|Default|GetWolf))
  (bind (_enemy _spawnarea_start _spawnarea_end) (Utilities|Struct|BreakEnemySpawn _wolf))
  (bind (_x _y _z) (Math|Vector|BreakVector _spawnarea_end))
  (bind (_x_2 _y_2 _z_2) (Math|Vector|BreakVector _spawnarea_start))
  (bind _returnvalue (Game|SpawnActorfromClass _enemy (Math|Transform|MakeTransform (Math|Vector|MakeVector (Math|Random|RandomFloatinRange _x_2 _x) (Math|Random|RandomFloatinRange _y_2 _y) (Math|Random|RandomFloatinRange _z_2 _z)) "0, 0, 0" (Variables|Default|GetScale)) "AlwaysSpawn" 0 0))
  (Pawn|SpawnDefaultController _returnvalue))

(fn SetWisp
  (bind _wisp (Variables|Default|GetWisp))
  (bind (_enemy _spawnarea_start _spawnarea_end) (Utilities|Struct|BreakEnemySpawn _wisp))
  (bind (_x _y _z) (Math|Vector|BreakVector _spawnarea_end))
  (bind (_x_2 _y_2 _z_2) (Math|Vector|BreakVector _spawnarea_start))
  (bind _returnvalue (Game|SpawnActorfromClass _enemy (Math|Transform|MakeTransform (Math|Vector|MakeVector (Math|Random|RandomFloatinRange _x_2 _x) (Math|Random|RandomFloatinRange _y_2 _y) (Math|Random|RandomFloatinRange _z_2 _z)) "0, 0, 0" (Variables|Default|GetScale)) "AlwaysSpawn" 0 0))
  (Pawn|SpawnDefaultController _returnvalue))

(fn SetWingRabbit
  (bind _rabbit (Variables|Default|GetRabbit))
  (bind (_enemy _spawnarea_start _spawnarea_end) (Utilities|Struct|BreakEnemySpawn _rabbit))
  (bind (_x _y _z) (Math|Vector|BreakVector _spawnarea_end))
  (bind (_x_2 _y_2 _z_2) (Math|Vector|BreakVector _spawnarea_start))
  (bind _returnvalue (Game|SpawnActorfromClass _enemy (Math|Transform|MakeTransform (Math|Vector|MakeVector (Math|Random|RandomFloatinRange _x_2 _x) (Math|Random|RandomFloatinRange _y_2 _y) (Math|Random|RandomFloatinRange _z_2 _z)) "0, 0, 0" (Variables|Default|GetScale)) "AlwaysSpawn" 0 0))
  (Pawn|SpawnDefaultController _returnvalue))

(fn SetLizzared
  (bind _lizzerd (Variables|Default|GetLizzerd))
  (bind (_enemy _spawnarea_start _spawnarea_end) (Utilities|Struct|BreakEnemySpawn _lizzerd))
  (bind (_x _y _z) (Math|Vector|BreakVector _spawnarea_end))
  (bind (_x_2 _y_2 _z_2) (Math|Vector|BreakVector _spawnarea_start))
  (bind _returnvalue (Game|SpawnActorfromClass _enemy (Math|Transform|MakeTransform (Math|Vector|MakeVector (Math|Random|RandomFloatinRange _x_2 _x) (Math|Random|RandomFloatinRange _y_2 _y) (Math|Random|RandomFloatinRange _z_2 _z)) "0, 0, 0" (Variables|Default|GetScale)) "AlwaysSpawn" 0 0))
  (Pawn|SpawnDefaultController _returnvalue))

(fn SetSpawn
  (bind _returnvalue (Game|SpawnActorfromClass "/Game/Enemy/Salamander/BP_Salamander.BP_Salamander_C" (Math|Transform|MakeTransform "-5800.000000,-5050.000000,640.000000" "0,56.000000, 0") "Undefined" 0 0))
  (Pawn|SpawnDefaultController _returnvalue))