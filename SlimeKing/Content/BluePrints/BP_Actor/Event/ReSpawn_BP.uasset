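; ReSpawn_BP is a trigger volume actor that sends player characters into their respawn logic when they touch it.
; On Box overlap, a sequence tries a cast to each of eight character classes, four regular and four tutorial variants, and calls HitRespawn on the match.
; The respawn behavior lives in each character; this actor only detects the overlap and forwards it.
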(event OnComponentBeginOverlap(Box)
  (params (OverlappedComponent :type Primitive%20Component%20Object%20Reference) (OtherActor :type Actor%20Object%20Reference) (OtherComp :type Primitive%20Component%20Object%20Reference) (OtherBodyIndex :type Integer) (bFromSweep :type Boolean) (SweepResult :type Hit%20Result%20Structure%20%28by%20ref%29))
  (Utilities|FlowControl|Sequence
    (:then_0
      (Default|HitRespawn (.AsBP%20Character (Utilities|Casting|CastToBP_Character OtherActor))))
    (:then_1
      (Default|HitRespawn (.AsBP%20Character%2002 (Utilities|Casting|CastToBP_Character_02 OtherActor))))
    (:then_2
      (Default|HitRespawn (.AsBP%20Character%2003 (Utilities|Casting|CastToBP_Character_03 OtherActor))))
    (:then_3
      (Default|HitRespawn (.AsBP%20Character%2004 (Utilities|Casting|CastToBP_Character_04 OtherActor))))
    (:then_4
      (Default|HitRespawn (.AsBP%20Character%20Turtrial (Utilities|Casting|CastToBP_Character_turtrial OtherActor))))
    (:then_5
      (Default|HitRespawn (.AsBP%20Character%2002%20Turtorial (Utilities|Casting|CastToBP_Character_02_Turtorial OtherActor))))
    (:then_6
      (Default|HitRespawn (.AsBP%20Character%2003%20Turtorial (Utilities|Casting|CastToBP_Character_03_Turtorial OtherActor))))
    (:then_7
      (Default|HitRespawn (.AsBP%20Character%2004%20Turtorial (Utilities|Casting|CastToBP_Character_04_Turtorial OtherActor))))))

(fn ConstructionScript)