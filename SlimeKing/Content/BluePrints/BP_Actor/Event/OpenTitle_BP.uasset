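; OpenTitle_BP is a trigger actor that loads the "title" level once all four tutorial characters have entered its Box.
; Box overlap casts the other actor to each tutorial character class and latches a matching boolean.
; Tick polls the four flags and calls OpenLevelByName when all are true.
; The flags are never cleared, so the characters need not be inside simultaneously.
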(event OnComponentBeginOverlap(Box)
  (params (OverlappedComponent :type Primitive%20Component%20Object%20Reference) (OtherActor :type Actor%20Object%20Reference) (OtherComp :type Primitive%20Component%20Object%20Reference) (OtherBodyIndex :type Integer) (bFromSweep :type Boolean) (SweepResult :type Hit%20Result%20Structure%20%28by%20ref%29))
  (Utilities|FlowControl|Sequence
    (:then_0
      (if (.bSuccess (Utilities|Casting|CastToBP_Character_turtrial OtherActor))
        (Variables|Default|SetNewVar_0 true)))
    (:then_1
      (if (.bSuccess (Utilities|Casting|CastToBP_Character_02_Turtorial OtherActor))
        (Variables|Default|SetNewVar_1 true)))
    (:then_2
      (if (.bSuccess (Utilities|Casting|CastToBP_Character_03_Turtorial OtherActor))
        (Variables|Default|SetNewVar_2 true)))
    (:then_3
      (if (.bSuccess (Utilities|Casting|CastToBP_Character_04_Turtorial OtherActor))
        (Variables|Default|SetNewVar_3 true)))))

(event EventBeginPlay)

(event Collision|EventActorBeginOverlap
  (params (OtherActor :type Actor%20Object%20Reference)))

(event EventTick
  (params (DeltaSeconds :type Float%20%28single-precision%29))
  (if (Variables|Default|GetNewVar_0)
    (if (Variables|Default|GetNewVar_1)
      (if (Variables|Default|GetNewVar_2)
        (if (Variables|Default|GetNewVar_3)
          (Game|OpenLevel(byName) "title"))))))

(fn ConstructionScript)