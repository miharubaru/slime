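; Enemy spawner actor that periodically repopulates the level with wolves, whisps, wing rabbits and lizards at random positions.
; Tick accumulates time, starting at the interval so the first wave is immediate, and each wave spawns two of each type.
; Per-type functions pick a point within that enemy's area bounds, always spawn and add a default controller; whisps ignore SpawnScale.
; Salamander and grass functions exist but are never called here.
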(event EventBeginPlay
  (Variables|Default|Settime (Variables|Default|GetspawnTimeInterval)) ; 開始後即スポーンするように
)

(event Collision|EventActorBeginOverlap
  (params (OtherActor :type Actor%20Object%20Reference)))

(event EventTick
  (params (DeltaSeconds :type Float%20%28single-precision%29))
  (bind _output_get (Variables|Default|Settime (+ DeltaSeconds (Variables|Default|Gettime))))
  (if (>= _output_get (Variables|Default|GetspawnTimeInterval)) ; time秒経過
    (CallFunction|SpawnWolf)
    (CallFunction|SpawnWhisp)
    (CallFunction|SpawnWingRabbit)
    (CallFunction|SpawnLizard)
    (CallFunction|SpawnWolf)
    (CallFunction|SpawnWhisp)
    (CallFunction|SpawnWingRabbit)
    (CallFunction|SpawnLizard)
    (Variables|Default|Settime 0.0)))

(fn ConstructionScript)

(fn SpawnWolf
  (bind _wolf (Variables|Default|Getwolf))
  (bind (_enemy _spawnarea_start _spawnarea_end) (Utilities|Struct|BreakEnemySpawn _wolf))
  (bind (_x _y _z) (Math|Vector|BreakVector _spawnarea_end))
  (bind (_x_2 _y_2 _z_2) (Math|Vector|BreakVector _spawnarea_start))
  (bind _returnvalue (Game|SpawnActorfromClass _enemy (Math|Transform|MakeTransform (Math|Vector|MakeVector (Math|Random|RandomFloatinRange _x_2 _x) (Math|Random|RandomFloatinRange _y_2 _y) (Math|Random|RandomFloatinRange _z_2 _z)) "0, 0, 0" (Variables|Default|GetspawnScale)) "AlwaysSpawn" 0 0))
  (Pawn|SpawnDefaultController _returnvalue))

(fn SpawnWhisp
  (bind _whisp (Variables|Default|Getwhisp))
  (bind (_enemy _spawnarea_start _spawnarea_end) (Utilities|Struct|BreakEnemySpawn _whisp))
  (bind (_x _y _z) (Math|Vector|BreakVector _spawnarea_end))
  (bind (_x_2 _y_2 _z_2) (Math|Vector|BreakVector _spawnarea_start))
  (bind _returnvalue (Game|SpawnActorfromClass _enemy (Math|Transform|MakeTransform (Math|Vector|MakeVector (Math|Random|RandomFloatinRange _x_2 _x) (Math|Random|RandomFloatinRange _y_2 _y) (Math|Random|RandomFloatinRange _z_2 _z))) "AlwaysSpawn" 0 0))
  (Pawn|SpawnDefaultController _returnvalue))

(fn SpawnWingRabbit
  (bind _wingrabbit (Variables|Default|GetwingRabbit))
  (bind (_enemy _spawnarea_start _spawnarea_end) (Utilities|Struct|BreakEnemySpawn _wingrabbit))
  (bind (_x _y _z) (Math|Vector|BreakVector _spawnarea_end))
  (bind (_x_2 _y_2 _z_2) (Math|Vector|BreakVector _spawnarea_start))
  (bind _returnvalue (Game|SpawnActorfromClass _enemy (Math|Transform|MakeTransform (Math|Vector|MakeVector (Math|Random|RandomFloatinRange _x_2 _x) (Math|Random|RandomFloatinRange _y_2 _y) (Math|Random|RandomFloatinRange _z_2 _z)) "0, 0, 0" (Variables|Default|GetspawnScale)) "AlwaysSpawn" 0 0))
  (Pawn|SpawnDefaultController _returnvalue))

(fn SpawnSalamander
  (bind _salamander (Variables|Default|Getsalamander))
  (bind (_enemy _spawnarea_start _spawnarea_end) (Utilities|Struct|BreakEnemySpawn _salamander))
  (bind (_x _y _z) (Math|Vector|BreakVector _spawnarea_end))
  (bind (_x_2 _y_2 _z_2) (Math|Vector|BreakVector _spawnarea_start))
  (bind _returnvalue (Game|SpawnActorfromClass _enemy (Math|Transform|MakeTransform (Math|Vector|MakeVector (Math|Random|RandomFloatinRange _x_2 _x) (Math|Random|RandomFloatinRange _y_2 _y) (Math|Random|RandomFloatinRange _z_2 _z)) "0, 0, 0" (Variables|Default|GetspawnScale)) "AlwaysSpawn" 0 0))
  (Pawn|SpawnDefaultController _returnvalue))

(fn SpawnLizard
  (bind _lizard (Variables|Default|Getlizard))
  (bind (_enemy _spawnarea_start _spawnarea_end) (Utilities|Struct|BreakEnemySpawn _lizard))
  (bind (_x _y _z) (Math|Vector|BreakVector _spawnarea_end))
  (bind (_x_2 _y_2 _z_2) (Math|Vector|BreakVector _spawnarea_start))
  (bind _returnvalue (Game|SpawnActorfromClass _enemy (Math|Transform|MakeTransform (Math|Vector|MakeVector (Math|Random|RandomFloatinRange _x_2 _x) (Math|Random|RandomFloatinRange _y_2 _y) (Math|Random|RandomFloatinRange _z_2 _z)) "0, 0, 0" (Variables|Default|GetspawnScale)) "AlwaysSpawn" 0 0))
  (Pawn|SpawnDefaultController _returnvalue))

(fn SpawnGrass
  (bind _grass (Variables|Default|GetGrass))
  (bind (_enemy _spawnarea_start _spawnarea_end) (Utilities|Struct|BreakEnemySpawn _grass))
  (bind (_x _y _z) (Math|Vector|BreakVector _spawnarea_end))
  (bind (_x_2 _y_2 _z_2) (Math|Vector|BreakVector _spawnarea_start))
  (bind _returnvalue (Game|SpawnActorfromClass _enemy (Math|Transform|MakeTransform (Math|Vector|MakeVector (Math|Random|RandomFloatinRange _x_2 _x) (Math|Random|RandomFloatinRange _y_2 _y) (Math|Random|RandomFloatinRange _z_2 _z)) "0, 0, 0" (Variables|Default|GetspawnScale)) "AlwaysSpawn" 0 0))
  (Pawn|SpawnDefaultController _returnvalue))