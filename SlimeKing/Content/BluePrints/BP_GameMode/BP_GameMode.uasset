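; BP_GameMode is a game mode Blueprint that adds a local player when play begins.
; BeginPlay calls CreatePlayer for controller ID 1 and spawns its player controller, which points to local multiplayer.
; An unconnected branch would spawn a scaled-up BP_Wolf at the parent Test2 actor's location at a set UI_BP GameTime, but it never runs.
; Tick and the construction script are empty.
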(event EventBeginPlay
  (Utilities|FlowControl|Sequence
    (:then_0
      (Class|GameplayStatics|CreatePlayer 1))))

(event EventTick
  (params (DeltaSeconds :type Float%20%28single-precision%29)))

(fn ConstructionScript)