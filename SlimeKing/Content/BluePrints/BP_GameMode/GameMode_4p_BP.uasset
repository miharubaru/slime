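; GameMode_4p_BP is a game mode Blueprint, apparently for four-player local play, with no active logic.
; A disconnected chain creates three extra players with controllers and stores them in separate arrays, BP2 to BP4.
; A second disconnected chain removes those players through nested loops, destroying their pawns.
; BeginPlay, the construction script and the AmeTime function are empty.
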(event EventBeginPlay)

(fn ConstructionScript)

(fn AmeTime)