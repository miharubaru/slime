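; Player-one slime character that grows with score and opens the result level on overlapping a larger player-two slime.
; AddScore functions add per-enemy points, rescale the mesh and copy the score to the game instance, while jumping costs score.
; AddItem stores Wolf, Wisp or WingRabbit item data from ActorTrace and arms a one-use ability: timed speed change, particles at player two's camera, or high jump.
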(event OnComponentBeginOverlap(Sphere)
  (params (OverlappedComponent :type Primitive%20Component%20Object%20Reference) (OtherActor :type Actor%20Object%20Reference) (OtherComp :type Primitive%20Component%20Object%20Reference) (OtherBodyIndex :type Integer) (bFromSweep :type Boolean) (SweepResult :type Hit%20Result%20Structure%20%28by%20ref%29))
  (bind _returnvalue (Game|GetPlayerCharacter 1))
  (bind _asbp_character_02 (Utilities|Casting|CastToBP_Character_02 _returnvalue))
  ;[1 1 1] SlimeBattle
  (if (.bSuccess (Utilities|Casting|CastToBP_Character_02 OtherActor))
    (Utilities|FlowControl|Sequence ; Player追加ここ
      (:then_0
        (bind _output_get (Variables|Default|SetSlimeScale (.z (Transformation|GetWorldScale (Variables|Character|GetMesh))))))
      (:then_1
        (bind _output_get_2 (Variables|/Game/BluePrints/BP_Character/BP_Character_02.BP_Character_02_C|SetSlimeScale_2 _asbp_character_02 (.z (Transformation|GetWorldScale (Variables|/Script/Engine.Character|GetMesh _asbp_character_02)))))))
    (if (< _output_get _output_get_2)
      (Game|OpenLevel(byName) "result"))))

(event EventBeginPlay
  ;[1 1 1] Score,Enlargement
  (Utilities|FlowControl|Sequence ; 敵のスコア/スライムの巨大化数値
    (:then_0
      (Variables|Default|Setscore_slime 1) ; 草のスコア
      (Variables|Default|SetScoreWisp 20) ; Wispのスコア
      (Variables|Default|SetScoreLizard 10) ; Lizardのスコア
      (Variables|Default|SetScoreWingRabbit 30)
      (Variables|Default|Setscore_wolf 40) ; ウルフのスコア/新しい敵はこの右に継ぎ足しok
    )
    (:then_1
      (Variables|Default|Setmagnification_score 80) ; スライムの大きくなるscoreの設定
      (Variables|Default|Setmagnification 0.2) ; スライムの大きくなる倍率
      (Variables|Default|Setmagnification_vector "1.000000,1.000000,1.000000") ; 巨大化に使うVector値。いじらなくてヨシ!
    )))

(event Input|ActionEvents|InputActionJump
  (params (Key :type Key%20Structure))
  ;[1 1 1] Controller
  (:Pressed
    (Utilities|FlowControl|Delay 0.5)
    (Character|Jump (Game|GetPlayerCharacter 0))
    (Utilities|FlowControl|Delay 1.5)
    (Variables|Default|SetScore (- (Variables|Default|GetScore) (Variables|Default|GetJumpScore)))))

(event Input|ActionEvents|InputActionAbility
  (params (Key :type Key%20Structure))
  (bind _charactermovement (Variables|Character|GetCharacterMovement))
  ;[1 1 1] Ability
  (:Pressed
    (Utilities|FlowControl|Sequence
      (:then_0
        (if (Variables|Default|GetWolfAbility)
          (CallFunction|SetWolf)
          (Utilities|FlowControl|Delay 3.0)
          (Variables|/Script/Engine.CharacterMovementComponent|SetMaxWalkSpeed _charactermovement 6e+02)
          (Variables|Default|SetWolfAbility false)
          (Variables|Default|SetHaveItem? false :!label _label)))
      (:then_1
        (if (Variables|Default|GetWispAbility)
          (CallFunction|SetWisp)
          (Variables|Default|SetWispAbility false)
          (goto _label)))
      (:then_2
        (if (Variables|Default|GetWingRabitAbility)
          (Components|Movement|StopMovementImmediately _charactermovement)
          (CallFunction|SetWingRabbit)
          (Utilities|FlowControl|Delay 0.1)
          (Variables|/Script/Engine.CharacterMovementComponent|SetJumpZVelocity _charactermovement 8e+02)
          (Variables|Default|SetWingRabitAbility false)
          (goto _label))))))

(event Input|AxisEvents|InputAxisMoveForward
  (params (AxisValue :type Float%20%28single-precision%29))
  (bind _returnvalue (Game|Player|GetPlayerPawn 0))
  ;[1 1 1] Controller
  (Pawn|Input|AddMovementInput _returnvalue (Math|Vector|GetForwardVector (Pawn|GetControlRotation _returnvalue :!class /Script/Engine.Pawn)) AxisValue false))

(event Input|AxisEvents|InputAxisMoveRight
  (params (AxisValue :type Float%20%28single-precision%29))
  (bind _returnvalue (Game|Player|GetPlayerPawn 0))
  ;[1 1 1] Controller
  (Pawn|Input|AddMovementInput _returnvalue (Math|Vector|GetRightVector (Pawn|GetControlRotation _returnvalue :!class /Script/Engine.Pawn)) AxisValue false))

(event Input|AxisEvents|InputAxisForcus
  (params (AxisValue :type Float%20%28single-precision%29))
  (bind _springarm (Variables|Default|GetSpringArm))
  ;[1 1 1] Comment
  (Variables|/Script/Engine.SpringArmComponent|SetTargetArmLength _springarm (+ (Variables|/Script/Engine.SpringArmComponent|GetTargetArmLength _springarm) (* AxisValue -1e+01))))

(event Input|AxisEvents|InputAxisTurn
  (params (AxisValue :type Float%20%28single-precision%29))
  ;[1 1 1] Controller
  (Pawn|Input|AddControllerYawInput (Game|GetPlayerCharacter 0) AxisValue))

(fn ConstructionScript)

(fn AddScore
  (bind _output_get (Variables|Default|SetScore (+ (Variables|Default|GetScore) (Variables|Default|Getscore_slime))))
  (Transformation|SetWorldScale3D (Variables|Character|GetMesh) (+ (Variables|Default|Getmagnification_vector) (* (/ _output_get (Variables|Default|Getmagnification_score)) (Variables|Default|Getmagnification))))
  (bind _asgame_instace_bp (Utilities|Casting|CastToGameInstace_BP (Game|GetGameInstance)))
  (Variables|/Game/BluePrints/BP_Wiedget/GameInstace_BP.GameInstace_BP_C|Setslime_1_score _asgame_instace_bp (Variables|Default|GetScore)))

(fn SetWingRabbit
  (Variables|/Script/Engine.CharacterMovementComponent|SetJumpZVelocity (Variables|Character|GetCharacterMovement) 1.6e+03)
  (Character|Jump (Game|GetPlayerCharacter 0)))

(fn AddScoreLizard
  (bind _output_get (Variables|Default|SetScore (+ (Variables|Default|GetScore) (Variables|Default|GetScoreLizard))))
  (Transformation|SetWorldScale3D (Variables|Character|GetMesh) (+ (Variables|Default|Getmagnification_vector) (* (/ _output_get (Variables|Default|Getmagnification_score)) (Variables|Default|Getmagnification))))
  (bind _asgame_instace_bp (Utilities|Casting|CastToGameInstace_BP (Game|GetGameInstance)))
  (Variables|/Game/BluePrints/BP_Wiedget/GameInstace_BP.GameInstace_BP_C|Setslime_1_score _asgame_instace_bp (Variables|Default|GetScore)))

(fn AddScoreWolf
  (bind _output_get (Variables|Default|SetScore (+ (Variables|Default|GetScore) (Variables|Default|Getscore_wolf))))
  (Transformation|SetWorldScale3D (Variables|Character|GetMesh) (+ (Variables|Default|Getmagnification_vector) (* (/ _output_get (Variables|Default|Getmagnification_score)) (Variables|Default|Getmagnification))))
  (bind _asgame_instace_bp (Utilities|Casting|CastToGameInstace_BP (Game|GetGameInstance)))
  (Variables|/Game/BluePrints/BP_Wiedget/GameInstace_BP.GameInstace_BP_C|Setslime_1_score _asgame_instace_bp (Variables|Default|GetScore)))

(fn AddScoreWisp
  (bind _output_get (Variables|Default|SetScore (+ (Variables|Default|GetScore) (Variables|Default|GetScoreWisp))))
  (Transformation|SetWorldScale3D (Variables|Character|GetMesh) (+ (Variables|Default|Getmagnification_vector) (* (/ _output_get (Variables|Default|Getmagnification_score)) (Variables|Default|Getmagnification))))
  (bind _asgame_instace_bp (Utilities|Casting|CastToGameInstace_BP (Game|GetGameInstance)))
  (Variables|/Game/BluePrints/BP_Wiedget/GameInstace_BP.GameInstace_BP_C|Setslime_1_score _asgame_instace_bp (Variables|Default|GetScore)))

(fn SetWolf
  (Variables|/Script/Engine.CharacterMovementComponent|SetMaxWalkSpeed (Variables|Character|GetCharacterMovement) (Variables|Default|Getspeed))
  (return))

(fn SetWisp
  (Effects|SpawnEmitteratLocation "/Game/Perticle/WhispParticle1.WhispParticle1" (Transformation|GetWorldLocation (Variables|/Game/BluePrints/BP_Character/BP_Character_02.BP_Character_02_C|GetCamera (.AsBP%20Character%2002 (Utilities|Casting|CastToBP_Character_02 (Game|GetPlayerCharacter 1)))))))

(fn AddScoreWingRabbit
  (bind _output_get (Variables|Default|SetScore (+ (Variables|Default|GetScore) (Variables|Default|GetScoreWingRabbit))))
  (Transformation|SetWorldScale3D (Variables|Character|GetMesh) (+ (Variables|Default|Getmagnification_vector) (* (/ _output_get (Variables|Default|Getmagnification_score)) (Variables|Default|Getmagnification))))
  (bind _asgame_instace_bp (Utilities|Casting|CastToGameInstace_BP (Game|GetGameInstance)))
  (Variables|/Game/BluePrints/BP_Wiedget/GameInstace_BP.GameInstace_BP_C|Setslime_1_score _asgame_instace_bp (Variables|Default|GetScore)))

(fn AddItem
  (bind _actortrace (Variables|Default|GetActorTrace))
  (bind _actortrace_2 (Variables|Default|GetActorTrace))
  (bind (_asbp_wolf _bsuccess) (Utilities|Casting|CastToBP_Wolf _actortrace))
  (bind (_aswing_rabbit _bsuccess_2) (Utilities|Casting|CastToWingRabbit _actortrace))
  (bind (_asbp_whisp _bsuccess_3) (Utilities|Casting|CastToBP_Whisp _actortrace))
  (bind (_aswing_rabbit_2 _bsuccess_4) (Utilities|Casting|CastToWingRabbit _actortrace_2))
  (bind (_asbp_wolf_2 _bsuccess_5) (Utilities|Casting|CastToBP_Wolf _actortrace_2))
  (bind (_asbp_whisp_2 _bsuccess_6) (Utilities|Casting|CastToBP_Whisp _actortrace_2))
  (if (Variables|Default|GetHaveItem?)
    (Variables|Default|SetWispAbility false)
    (Variables|Default|SetWolfAbility false)
    (Variables|Default|SetWingRabitAbility false)
    (Utilities|FlowControl|Sequence
      (:then_0
        (if _bsuccess
          (Utilities|Array|Add (Variables|Default|GetInventory) (Variables|/Game/BluePrints/BP_Inventory/Inventory/test.test_C|GetItemData _asbp_wolf))
          (Variables|Default|SetWolfAbility true)
          (Variables|Default|SetHaveItem? true :!label _label)
          (return)))
      (:then_1
        (if _bsuccess_3
          (Utilities|Array|Add (Variables|Default|GetInventory) (Variables|/Game/BluePrints/BP_Inventory/Inventory/test.test_C|GetItemData _asbp_whisp))
          (Variables|Default|SetWispAbility true)
          (goto _label)))
      (:then_2
        (if _bsuccess_2
          (Utilities|Array|Add (Variables|Default|GetInventory) (Variables|/Game/BluePrints/BP_Inventory/Inventory/test.test_C|GetItemData _aswing_rabbit))
          (Variables|Default|SetWingRabitAbility true)
          (goto _label))))
    (else
      (Utilities|FlowControl|Sequence
        (:then_0
          (if _bsuccess_5
            (Utilities|Array|Add (Variables|Default|GetInventory) (Variables|/Game/BluePrints/BP_Inventory/Inventory/test.test_C|GetItemData _asbp_wolf_2))
            (Variables|Default|SetWolfAbility true)
            (Variables|Default|SetHaveItem? true :!label _label_2)
            (return)))
        (:then_1
          (if _bsuccess_6
            (Utilities|Array|Add (Variables|Default|GetInventory) (Variables|/Game/BluePrints/BP_Inventory/Inventory/test.test_C|GetItemData _asbp_whisp_2))
            (Variables|Default|SetWispAbility true)
            (goto _label_2)))
        (:then_2
          (if _bsuccess_4
            (Utilities|Array|Add (Variables|Default|GetInventory) (Variables|/Game/BluePrints/BP_Inventory/Inventory/test.test_C|GetItemData _aswing_rabbit_2))
            (Variables|Default|SetWingRabitAbility true)
            (goto _label_2)))))))

(fn ScoreInstance
  (bind _asgame_instace_bp (Utilities|Casting|CastToGameInstace_BP (Game|GetGameInstance)))
  (Variables|/Game/BluePrints/BP_Wiedget/GameInstace_BP.GameInstace_BP_C|Setslime_1_score _asgame_instace_bp (Variables|Default|GetScore)))

(fn ScoreGameInstance
  (bind _asgame_instace_bp (Utilities|Casting|CastToGameInstace_BP (Game|GetGameInstance)))
  (bind _output_get (Variables|/Game/BluePrints/BP_Wiedget/GameInstace_BP.GameInstace_BP_C|Setslime_1_score _asgame_instace_bp (Variables|Default|GetScore)))
  (Development|PrintText (Utilities|Text|ToText(Integer) _output_get)))