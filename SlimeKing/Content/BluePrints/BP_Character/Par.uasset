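; Par is a Blueprint that ends the current level by opening the "result" level once at least three of its four BP1 to BP4 conditions are true.
; Every Tick, a Sequence runs four nested Branch chains, one for each possible combination of three conditions, all wired into a shared OpenLevelByName call.
; Nothing in its graphs sets these conditions, and the construction script is empty.
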(event EventTick
  (params (DeltaSeconds :type Float%20%28single-precision%29))
  (Utilities|FlowControl|Sequence
    (:then_0
      ;[1 1 1] 4
      (if (Variables|Default|GetBP1)
        (if (Variables|Default|GetBP2)
          (if (Variables|Default|GetBP3)
            (Game|OpenLevel(byName) "result" :!label _label)))))
    (:then_1
      ;[1 1 1] 3
      (if (Variables|Default|GetBP1)
        (if (Variables|Default|GetBP2)
          (if (Variables|Default|GetBP4)
            (goto _label)))))
    (:then_2
      ;[1 1 1] 2
      (if (Variables|Default|GetBP1)
        (if (Variables|Default|GetBP3)
          (if (Variables|Default|GetBP4)
            (goto _label)))))
    (:then_3
      ;[1 1 1] 1
      (if (Variables|Default|GetBP2)
        (if (Variables|Default|GetBP3)
          (if (Variables|Default|GetBP4)
            (goto _label)))))))

(fn ConstructionScript)