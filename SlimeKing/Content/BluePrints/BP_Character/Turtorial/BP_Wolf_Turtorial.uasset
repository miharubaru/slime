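; BP_Wolf_Turtorial is an AI wolf pawn for the tutorial that grants the wolf ability to the player characters.
; When PawnSensing sees one of the four tutorial character classes, it writes that pawn to the blackboard Player key.
; When its Box overlaps one of those characters, it resets that character's abilities, sets its wolf ability flag and destroys itself.
; Each character class is handled by a separate cast on a Sequence pin.
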(event OnSeePawn(PawnSensing)
  (params (Pawn :type Pawn%20Object%20Reference))
  (bind _returnvalue (Utilities|Name|MakeLiteralName "Player"))
  (bind _self self)
  (bind _returnvalue_2 (AI|GetBlackboard _self))
  (Utilities|FlowControl|Sequence
    (:then_0
      (bind _asbp_character_turtrial (Utilities|Casting|CastToBP_Character_turtrial Pawn))
      (AI|Components|Blackboard|SetValueasObject _returnvalue_2 _returnvalue _asbp_character_turtrial))
    (:then_1
      (bind _asbp_character_02_turtorial (Utilities|Casting|CastToBP_Character_02_Turtorial Pawn))
      (AI|Components|Blackboard|SetValueasObject _returnvalue_2 _returnvalue _asbp_character_02_turtorial))
    (:then_2
      (bind _asbp_character_03_turtorial (Utilities|Casting|CastToBP_Character_03_Turtorial Pawn))
      (AI|Components|Blackboard|SetValueasObject _returnvalue_2 _returnvalue _asbp_character_03_turtorial))
    (:then_3
      (bind _asbp_character_04_turtorial (Utilities|Casting|CastToBP_Character_04_Turtorial Pawn))
      (AI|Components|Blackboard|SetValueasObject _returnvalue_2 _returnvalue _asbp_character_04_turtorial))))

(event OnComponentBeginOverlap(Box)
  (params (OverlappedComponent :type Primitive%20Component%20Object%20Reference) (OtherActor :type Actor%20Object%20Reference) (OtherComp :type Primitive%20Component%20Object%20Reference) (OtherBodyIndex :type Integer) (bFromSweep :type Boolean) (SweepResult :type Hit%20Result%20Structure%20%28by%20ref%29))
  (bind (_asbp_character_turtrial _bsuccess) (Utilities|Casting|CastToBP_Character_turtrial OtherActor))
  (bind (_asbp_character_02_turtorial _bsuccess_2) (Utilities|Casting|CastToBP_Character_02_Turtorial OtherActor))
  (bind (_asbp_character_03_turtorial _bsuccess_3) (Utilities|Casting|CastToBP_Character_03_Turtorial OtherActor))
  (bind (_asbp_character_04_turtorial _bsuccess_4) (Utilities|Casting|CastToBP_Character_04_Turtorial OtherActor))
  (Utilities|FlowControl|Sequence
    (:then_0
      (if _bsuccess
        (Default|AbilityRisset _asbp_character_turtrial)
        (Variables|/Game/BluePrints/BP_Character/Turtorial/BP_Character_turtrial.BP_Character_turtrial_C|SetWolfAbility _asbp_character_turtrial true)
        (Actor|DestroyActor :!label _label)))
    (:then_1
      (if _bsuccess_2
        (Default|AbilityRisset _asbp_character_02_turtorial)
        (Variables|/Game/BluePrints/BP_Character/Turtorial/BP_Character_02_Turtorial.BP_Character_02_Turtorial_C|SetWolfAbirity2 _asbp_character_02_turtorial true)
        (goto _label)))
    (:then_2
      (if _bsuccess_3
        (Default|AbilityRisset _asbp_character_03_turtorial)
        (Variables|/Game/BluePrints/BP_Character/Turtorial/BP_Character_03_Turtorial.BP_Character_03_Turtorial_C|SetWolfAbility _asbp_character_03_turtorial true)
        (goto _label)))
    (:then_3
      (if _bsuccess_4
        (Default|AbilityRisset _asbp_character_04_turtorial)
        (Variables|/Game/BluePrints/BP_Character/Turtorial/BP_Character_04_Turtorial.BP_Character_04_Turtorial_C|SetWolfAbility _asbp_character_04_turtorial true)
        (goto _label)))))

(event EventBeginPlay)

(fn ConstructionScript)