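; BP_Lizard_Turtorial is a tutorial lizard actor that disappears when a tutorial player character touches it.
; Its StaticMesh begin-overlap event runs a sequence of casts against the four tutorial character classes, each leading to DestroyActor.
; LizardScoreBP1 and LizardScoreBP2 add lizard score to non-tutorial characters of players 0 and 1, but nothing in this Blueprint calls them.
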(event OnComponentBeginOverlap(StaticMesh)
  (params (OverlappedComponent :type Primitive%20Component%20Object%20Reference) (OtherActor :type Actor%20Object%20Reference) (OtherComp :type Primitive%20Component%20Object%20Reference) (OtherBodyIndex :type Integer) (bFromSweep :type Boolean) (SweepResult :type Hit%20Result%20Structure%20%28by%20ref%29))
  (Utilities|FlowControl|Sequence
    (:then_0
      (if (.bSuccess (Utilities|Casting|CastToBP_Character_turtrial OtherActor))
        (Actor|DestroyActor :!label _label)))
    (:then_1
      (if (.bSuccess (Utilities|Casting|CastToBP_Character_02_Turtorial OtherActor))
        (goto _label)))
    (:then_2
      (if (.bSuccess (Utilities|Casting|CastToBP_Character_03_Turtorial OtherActor))
        (goto _label)))
    (:then_3
      (if (.bSuccess (Utilities|Casting|CastToBP_Character_04_Turtorial OtherActor))
        (goto _label)))))

(event EventBeginPlay)

(event Collision|EventActorBeginOverlap
  (params (OtherActor :type Actor%20Object%20Reference)))

(event EventTick
  (params (DeltaSeconds :type Float%20%28single-precision%29)))

(fn ConstructionScript)

(fn LizardScoreBP1
  (bind _asbp_character (Utilities|Casting|CastToBP_Character (Game|GetPlayerCharacter 0)))
  (Default|AddScoreLizard _asbp_character))

(fn LizardScoreBP2
  (bind _asbp_character_02 (Utilities|Casting|CastToBP_Character_02 (Game|GetPlayerCharacter 1)))
  (Default|AddScoreLizard _asbp_character_02))