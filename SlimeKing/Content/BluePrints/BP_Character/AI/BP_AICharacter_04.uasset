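; AI slime character paired with player 4 that awards split-slime score to whichever of the four player characters touches it, then destroys itself.
; PawnSensing writes any sighted BP_Character_04 to the blackboard's Player key.
; It also carries player-style functions, uncalled in its event graph, for score-driven mesh growth, Slime1Score saving, creature abilities and child-slime spawning.
; Several of these use hard-coded player indices 0 or 1.
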(event OnComponentBeginOverlap(Sphere)
  (params (OverlappedComponent :type Primitive%20Component%20Object%20Reference) (OtherActor :type Actor%20Object%20Reference) (OtherComp :type Primitive%20Component%20Object%20Reference) (OtherBodyIndex :type Integer) (bFromSweep :type Boolean) (SweepResult :type Hit%20Result%20Structure%20%28by%20ref%29))
  (bind (_asbp_character_02 _bsuccess) (Utilities|Casting|CastToBP_Character_02 OtherActor))
  (bind (_asbp_character _bsuccess_2) (Utilities|Casting|CastToBP_Character OtherActor))
  (bind (_asbp_character_03 _bsuccess_3) (Utilities|Casting|CastToBP_Character_03 OtherActor))
  (bind (_asbp_character_04 _bsuccess_4) (Utilities|Casting|CastToBP_Character_04 OtherActor))
  (Utilities|FlowControl|Sequence
    (:then_0
      (if _bsuccess_2
        (Default|AddScoreSplitSlime _asbp_character)
        (Actor|DestroyActor :!label _label)))
    (:then_1
      (if _bsuccess
        (Default|AddScoreSplitSlime _asbp_character_02)
        (goto _label)))
    (:then_2
      (if _bsuccess_3
        (Default|AddScoreSplitSlime _asbp_character_03)
        (goto _label)))
    (:then_3
      (if _bsuccess_4
        (Default|AddScoreSplitSlime _asbp_character_04)
        (goto _label)))))

(event OnSeePawn(PawnSensing1)
  (params (Pawn :type Pawn%20Object%20Reference))
  (bind _asbp_character_04 (Utilities|Casting|CastToBP_Character_04 Pawn))
  (AI|Components|Blackboard|SetValueasObject (AI|GetBlackboard self) (Utilities|Name|MakeLiteralName "Player") _asbp_character_04))

(fn ConstructionScript)

(fn AddScore
  (bind _output_get (Variables|Default|SetScore (+ (Variables|Default|GetScore) (Variables|Default|Getscore_slime))))
  (Transformation|SetWorldScale3D (Variables|Character|GetMesh) (+ (Variables|Default|Getmagnification_vector) (* (/ _output_get (Variables|Default|Getmagnification_score)) (Variables|Default|Getmagnification))))
  (bind _asgame_instace_bp (Utilities|Casting|CastToGameInstace_BP (Game|GetGameInstance)))
  (Variables|/Game/BluePrints/BP_Wiedget/GameInstace_BP.GameInstace_BP_C|Setslime_1_score _asgame_instace_bp (Variables|Default|GetScore)))

(fn SetWingRabbit
  (Variables|/Script/Engine.CharacterMovementComponent|SetJumpZVelocity (Variables|Character|GetCharacterMovement) 1.6e+03)
  (Character|Jump (Game|GetPlayerCharacter 0)))

(fn AddScoreLizard
  (bind _output_get (Variables|Default|SetScore (+ (Variables|Default|GetScore) (Variables|Default|GetScoreLizard))))
  (Transformation|SetWorldScale3D (Variables|Character|GetMesh) (+ (Variables|Default|Getmagnification_vector) (* (/ _output_get (Variables|Default|Getmagnification_score)) (Variables|Default|Getmagnification))))
  (bind _asgame_instace_bp (Utilities|Casting|CastToGameInstace_BP (Game|GetGameInstance)))
  (Variables|/Game/BluePrints/BP_Wiedget/GameInstace_BP.GameInstace_BP_C|Setslime_1_score _asgame_instace_bp (Variables|Default|GetScore)))

(fn AddScoreWolf
  (bind _output_get (Variables|Default|SetScore (+ (Variables|Default|GetScore) (Variables|Default|Getscore_wolf))))
  (Transformation|SetWorldScale3D (Variables|Character|GetMesh) (+ (Variables|Default|Getmagnification_vector) (* (/ _output_get (Variables|Default|Getmagnification_score)) (Variables|Default|Getmagnification))))
  (bind _asgame_instace_bp (Utilities|Casting|CastToGameInstace_BP (Game|GetGameInstance)))
  (Variables|/Game/BluePrints/BP_Wiedget/GameInstace_BP.GameInstace_BP_C|Setslime_1_score _asgame_instace_bp (Variables|Default|GetScore))
  (Audio|PlaySoundatLocation "/Game/Sounds/03_Slime_Acquired.03_Slime_Acquired" (Transformation|GetActorLocation (Game|GetPlayerCharacter 0)) "0, 0, 0" 1.0 1.0 0.0 "/Game/Sounds/NewSoundAttenuation.NewSoundAttenuation" 0 0))

(fn AddScoreWisp
  (bind _output_get (Variables|Default|SetScore (+ (Variables|Default|GetScore) (Variables|Default|GetScoreWisp))))
  (Transformation|SetWorldScale3D (Variables|Character|GetMesh) (+ (Variables|Default|Getmagnification_vector) (* (/ _output_get (Variables|Default|Getmagnification_score)) (Variables|Default|Getmagnification))))
  (bind _asgame_instace_bp (Utilities|Casting|CastToGameInstace_BP (Game|GetGameInstance)))
  (Variables|/Game/BluePrints/BP_Wiedget/GameInstace_BP.GameInstace_BP_C|Setslime_1_score _asgame_instace_bp (Variables|Default|GetScore))
  (Audio|PlaySoundatLocation "/Game/Sounds/03_Slime_Acquired.03_Slime_Acquired" (Transformation|GetActorLocation (Game|GetPlayerCharacter 0)) "0, 0, 0" 1.0 1.0 0.0 "/Game/Sounds/NewSoundAttenuation.NewSoundAttenuation" 0 0))

(fn SetWolf
  (Variables|/Script/Engine.CharacterMovementComponent|SetMaxWalkSpeed (Variables|Character|GetCharacterMovement) (Variables|Default|Getspeed))
  (return))

(fn SetWisp
  (Effects|SpawnEmitteratLocation "/Game/Perticle/WhispParticle1.WhispParticle1" (Transformation|GetWorldLocation (Variables|/Game/BluePrints/BP_Character/BP_Character_02.BP_Character_02_C|GetCamera (.AsBP%20Character%2002 (Utilities|Casting|CastToBP_Character_02 (Game|GetPlayerCharacter 1)))))))

(fn AddScoreWingRabbit
  (bind _output_get (Variables|Default|SetScore (+ (Variables|Default|GetScore) (Variables|Default|GetScoreWingRabbit))))
  (Transformation|SetWorldScale3D (Variables|Character|GetMesh) (+ (Variables|Default|Getmagnification_vector) (* (/ _output_get (Variables|Default|Getmagnification_score)) (Variables|Default|Getmagnification))))
  (bind _asgame_instace_bp (Utilities|Casting|CastToGameInstace_BP (Game|GetGameInstance)))
  (Variables|/Game/BluePrints/BP_Wiedget/GameInstace_BP.GameInstace_BP_C|Setslime_1_score _asgame_instace_bp (Variables|Default|GetScore))
  (Audio|PlaySoundatLocation "/Game/Sounds/03_Slime_Acquired.03_Slime_Acquired" (Transformation|GetActorLocation (Game|GetPlayerCharacter 0)) "0, 0, 0" 1.0 1.0 0.0 "/Game/Sounds/NewSoundAttenuation.NewSoundAttenuation" 0 0))

(fn AddItem
  (bind _actortrace (Variables|Default|GetActorTrace))
  (bind _actortrace_2 (Variables|Default|GetActorTrace))
  (bind (_asbp_wolf _bsuccess) (Utilities|Casting|CastToBP_Wolf _actortrace))
  (bind (_aswing_rabbit _bsuccess_2) (Utilities|Casting|CastToWingRabbit _actortrace))
  (bind (_asbp_whisp _bsuccess_3) (Utilities|Casting|CastToBP_Whisp _actortrace))
  (bind (_aswing_rabbit_2 _bsuccess_4) (Utilities|Casting|CastToWingRabbit _actortrace_2))
  (bind (_asbp_wolf_2 _bsuccess_5) (Utilities|Casting|CastToBP_Wolf _actortrace_2))
  (bind (_asbp_whisp_2 _bsuccess_6) (Utilities|Casting|CastToBP_Whisp _actortrace_2))
  (if (Variables|Default|GetHaveItem?)
    (Variables|Default|SetWispAbility false)
    (Variables|Default|SetWolfAbility false)
    (Variables|Default|SetWingRabitAbility false)
    (Utilities|FlowControl|Sequence
      (:then_0
        (if _bsuccess
          (Utilities|Array|Add (Variables|Default|GetInventory) (Variables|/Game/BluePrints/BP_Inventory/Inventory/test.test_C|GetItemData _asbp_wolf))
          (Variables|Default|SetWolfAbility true)
          (Variables|Default|SetHaveItem? true :!label _label)
          (return)))
      (:then_1
        (if _bsuccess_3
          (Utilities|Array|Add (Variables|Default|GetInventory) (Variables|/Game/BluePrints/BP_Inventory/Inventory/test.test_C|GetItemData _asbp_whisp))
          (Variables|Default|SetWispAbility true)
          (goto _label)))
      (:then_2
        (if _bsuccess_2
          (Utilities|Array|Add (Variables|Default|GetInventory) (Variables|/Game/BluePrints/BP_Inventory/Inventory/test.test_C|GetItemData _aswing_rabbit))
          (Variables|Default|SetWingRabitAbility true)
          (goto _label))))
    (else
      (Utilities|FlowControl|Sequence
        (:then_0
          (if _bsuccess_5
            (Utilities|Array|Add (Variables|Default|GetInventory) (Variables|/Game/BluePrints/BP_Inventory/Inventory/test.test_C|GetItemData _asbp_wolf_2))
            (Variables|Default|SetWolfAbility true)
            (Variables|Default|SetHaveItem? true :!label _label_2)
            (return)))
        (:then_1
          (if _bsuccess_6
            (Utilities|Array|Add (Variables|Default|GetInventory) (Variables|/Game/BluePrints/BP_Inventory/Inventory/test.test_C|GetItemData _asbp_whisp_2))
            (Variables|Default|SetWispAbility true)
            (goto _label_2)))
        (:then_2
          (if _bsuccess_4
            (Utilities|Array|Add (Variables|Default|GetInventory) (Variables|/Game/BluePrints/BP_Inventory/Inventory/test.test_C|GetItemData _aswing_rabbit_2))
            (Variables|Default|SetWingRabitAbility true)
            (goto _label_2)))))))

(fn ScoreInstance
  (bind _asgame_instace_bp (Utilities|Casting|CastToGameInstace_BP (Game|GetGameInstance)))
  (Variables|/Game/BluePrints/BP_Wiedget/GameInstace_BP.GameInstace_BP_C|Setslime_1_score _asgame_instace_bp (Variables|Default|GetScore)))

(fn ScoreGameInstance
  (bind _asgame_instace_bp (Utilities|Casting|CastToGameInstace_BP (Game|GetGameInstance)))
  (bind _output_get (Variables|/Game/BluePrints/BP_Wiedget/GameInstace_BP.GameInstace_BP_C|Setslime_1_score _asgame_instace_bp (Variables|Default|GetScore)))
  (Development|PrintText (Utilities|Text|ToText(Integer) _output_get)))

(fn SplitSlime
  (bind _returnvalue (Game|SpawnActorfromClass "/Game/BluePrints/BP_Character/AI/BP_Character_Child.BP_Character_Child_C" (Math|Transform|MakeTransform (Math|Random|RandomPointinBoundingBox (Transformation|GetWorldLocation (Variables|Character|GetMesh)) (Math|Vector|MakeVector (Math|Random|RandomFloatinRange 5e+02 5e+02) (Math|Random|RandomFloatinRange -5e+02 5e+02) 0.0))) "Undefined" 0 0))
  (Pawn|SpawnDefaultController _returnvalue))

(fn JumpUseScore
  (Variables|Default|SetScore (- (Variables|Default|GetScore) (Variables|Default|GetJumpScore))))

(fn AbilityWalkSpeed
  (Variables|/Script/Engine.CharacterMovementComponent|SetMaxWalkSpeed (Variables|Character|GetCharacterMovement) 6e+02))

(fn AbilityJumpStetas
  (Variables|/Script/Engine.CharacterMovementComponent|SetJumpZVelocity (Variables|Character|GetCharacterMovement) 8e+02))

(fn WingRabbitSound
  (Audio|PlaySoundatLocation "/Game/Sounds/14_SlimeWing_Descent.14_SlimeWing_Descent" (Transformation|GetActorLocation (Game|GetPlayerCharacter 0)) "0, 0, 0" 1.0 1.0 0.0 0 0 0) ; SlimeWing_Descent
)