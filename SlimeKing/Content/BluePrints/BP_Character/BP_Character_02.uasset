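; BP_Character_02 is a slime character that grows by scoring and can lose to player 0's slime (BP_Character).
; Grass and wolf functions add to Score and rescale the mesh from it, while AddScoreWisp stores its sum in ScoreWisp2 instead.
; On sphere overlap with BP_Character, it compares mesh scales, and if smaller hides itself and opens the result level.
; Helpers add inventory items, boost walk speed and spawn wisp particles.
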(event OnComponentBeginOverlap(Sphere)
  (params (OverlappedComponent :type Primitive%20Component%20Object%20Reference) (OtherActor :type Actor%20Object%20Reference) (OtherComp :type Primitive%20Component%20Object%20Reference) (OtherBodyIndex :type Integer) (bFromSweep :type Boolean) (SweepResult :type Hit%20Result%20Structure%20%28by%20ref%29))
  (bind _returnvalue (Game|GetPlayerCharacter 0))
  (bind _asbp_character (Utilities|Casting|CastToBP_Character _returnvalue))
  (if (.bSuccess (Utilities|Casting|CastToBP_Character OtherActor))
    (Utilities|FlowControl|Sequence
      (:then_0
        (bind _output_get (Variables|Default|SetSlimeScale_2 (.z (Transformation|GetWorldScale (Variables|Character|GetMesh))))))
      (:then_1
        (bind _output_get_2 (Variables|/Game/BluePrints/BP_Character/BP_Character.BP_Character_C|SetSlimeScale _asbp_character (.z (Transformation|GetWorldScale (Variables|/Script/Engine.Character|GetMesh _asbp_character)))))))
    (if (< _output_get _output_get_2)
      (Rendering|SetVisibility (Variables|Character|GetMesh) false false)
      (Rendering|SetVisibility (Variables|Default|GetSphere) false false)
      (Rendering|SetVisibility (Variables|Collision|GetCapsuleComponent) false false)
      (Game|OpenLevel(byName) "result"))))

(event EventBeginPlay
  (Utilities|FlowControl|Sequence
    (:then_0
      (Variables|Default|Setscore_grass_2 1)
      (Variables|Default|Setscore_wolf_2 5))
    (:then_1
      (Variables|Default|Setmagnification_score_2 30) ; スライムの大きくなるscoreの設定
      (Variables|Default|Setmagnification_2 0.2) ; スライムの大きくなる倍率
      (Variables|Default|Setmagnification_vector_2 "1.000000,1.000000,1.000000"))))

(fn ConstructionScript)

(fn AddScore
  (bind _output_get (Variables|Default|SetScore (+ (Variables|Default|GetScore) (Variables|Default|Getscore_grass_2))))
  (Transformation|SetWorldScale3D (Variables|Character|GetMesh) (+ (Variables|Default|Getmagnification_vector_2) (* (/ _output_get (Variables|Default|Getmagnification_score_2)) (Variables|Default|Getmagnification_2)))))

(fn AddScoreWolf
  (bind _output_get (Variables|Default|SetScore (+ (Variables|Default|GetScore) (Variables|Default|Getscore_wolf_2))))
  (Transformation|SetWorldScale3D (Variables|Character|GetMesh) (+ (Variables|Default|Getmagnification_vector_2) (* (/ _output_get (Variables|Default|Getmagnification_score_2)) (Variables|Default|Getmagnification_2)))))

(fn AddItem
  (bind _astest (Utilities|Casting|CastTotest (Variables|Default|GetActorTrace)))
  (Utilities|Array|Add (Variables|Default|GetInventory) (Variables|/Game/BluePrints/BP_Inventory/Inventory/test.test_C|GetItemData _astest))
  (return))

(fn SetWolf
  (Variables|/Script/Engine.CharacterMovementComponent|SetMaxWalkSpeed (Variables|Character|GetCharacterMovement) 5e+03)
  (return))

(fn AddScoreWisp
  (bind _output_get (Variables|Default|SetScoreWisp2 (+ (Variables|Default|GetScore) (Variables|Default|GetScoreWisp2))))
  (Transformation|SetWorldScale3D (Variables|Character|GetMesh) (+ (Variables|Default|Getmagnification_vector_2) (* (/ _output_get (Variables|Default|Getmagnification_score_2)) (Variables|Default|Getmagnification_2)))))

(fn SetWisp
  (Effects|SpawnEmitteratLocation "/Game/Goto/Whisp/WhispParticle.WhispParticle" (Transformation|GetWorldLocation (Variables|Character|GetMesh))))