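; Player 1's slime character, which grows with score, gains one-shot abilities and battles BP_Character_02.
; AddScore functions add per-enemy points and rescale the mesh, while jumping deducts score.
; AddItem records Wolf, Wisp or WingRabbit pickups, enabling a timed speed change, particle burst or high jump.
; Overlapping the rival while smaller opens the result level; Tick flip-flops the inventory widget every frame.
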(event OnComponentBeginOverlap(Sphere)
  (params (OverlappedComponent :type Primitive%20Component%20Object%20Reference) (OtherActor :type Actor%20Object%20Reference) (OtherComp :type Primitive%20Component%20Object%20Reference) (OtherBodyIndex :type Integer) (bFromSweep :type Boolean) (SweepResult :type Hit%20Result%20Structure%20%28by%20ref%29))
  (bind _returnvalue (Game|GetPlayerCharacter 1))
  (bind _asbp_character_02 (Utilities|Casting|CastToBP_Character_02 _returnvalue))
  ;[1 1 1] SlimeBattle
  (if (.bSuccess (Utilities|Casting|CastToBP_Character_02 OtherActor))
    (Utilities|FlowControl|Sequence ; Player追加ここ
      (:then_0
        (bind _output_get (Variables|Default|SetSlimeScale (.z (Transformation|GetWorldScale (Variables|Character|GetMesh))))))
      (:then_1
        (bind _output_get_2 (Variables|/Game/BluePrints/BP_Character/BP_Character_02.BP_Character_02_C|SetSlimeScale_2 _asbp_character_02 (.z (Transformation|GetWorldScale (Variables|/Script/Engine.Character|GetMesh _asbp_character_02)))))))
    (if (< _output_get _output_get_2)
      (Rendering|SetVisibility (Variables|Character|GetMesh) false false)
      (Rendering|SetVisibility (Variables|Default|GetSphere) false false)
      (Rendering|SetVisibility (Variables|Collision|GetCapsuleComponent) false false)
      (Game|OpenLevel(byName) "result"))))

(event EventBeginPlay
  ;[1 1 1] Score,Enlargement
  (Utilities|FlowControl|Sequence ; 敵のスコア/スライムの巨大化数値
    (:then_0
      (Variables|Default|Setscore_slime 1) ; 草のスコア
      (Variables|Default|SetScoreWisp 5) ; Wispのスコア
      (Variables|Default|SetScoreLizard 5) ; Lizardのスコア
      (Variables|Default|SetScoreWingRabbit 10)
      (Variables|Default|Setscore_wolf 5) ; ウルフのスコア/新しい敵はこの右に継ぎ足しok
    )
    (:then_1
      (Variables|Default|Setmagnification_score 30) ; スライムの大きくなるscoreの設定
      (Variables|Default|Setmagnification 0.2) ; スライムの大きくなる倍率
      (Variables|Default|Setmagnification_vector "1.000000,1.000000,1.000000") ; 巨大化に使うVector値。いじらなくてヨシ!
    )))

(event EventTick
  (params (DeltaSeconds :type Float%20%28single-precision%29))
  (bind _returnvalue (Game|GetPlayerController 0))
  ;[1 1 1] Inventory
  (Utilities|FlowControl|FlipFlop
    (:A
      (bind _returnvalue_2 (UserInterface|CreateWidget "/Game/BluePrints/BP_Inventory/Inventory/Inventory.Inventory_C" _returnvalue))
      (bind _output_get (Variables|Default|SetInventryRef _returnvalue_2))
      (UserInterface|Viewport|AddtoViewport _output_get 0)
      (Variables|/Script/Engine.PlayerController|SetbShowMouseCursor _returnvalue false)
      (Input|SetInputModeGameandUI _returnvalue _output_get "DoNotLock" true))
    (:B
      (Widget|RemovefromParent (Variables|Default|GetInventryRef))
      (Variables|/Script/Engine.PlayerController|SetbShowMouseCursor _returnvalue false)
      (Input|SetInputModeGameOnly _returnvalue))))

(event Input|ActionEvents|InputActionJump
  (params (Key :type Key%20Structure :default "None"))
  ;[1 1 1] Controller
  (:Pressed
    (Utilities|FlowControl|Delay 0.5)
    (Character|Jump (Game|GetPlayerCharacter 0))
    (Utilities|FlowControl|Delay 1.5)
    (Variables|Default|SetScore (- (Variables|Default|GetScore) (Variables|Default|GetJumpScore)))))

(event Input|ActionEvents|InputActionAbility
  (params (Key :type Key%20Structure :default "None"))
  ;[1 1 1] Ability
  (:Pressed
    (Utilities|FlowControl|Sequence
      (:then_0
        (if (Variables|Default|GetWolfAbility)
          (CallFunction|SetWolf)
          (Utilities|FlowControl|Delay 3.0)
          (Variables|/Script/Engine.CharacterMovementComponent|SetMaxWalkSpeed (Variables|Character|GetCharacterMovement) 6e+02)
          (CallFunction|RefreshItem)
          (Variables|Default|SetWolfAbility false)))
      (:then_1
        (if (Variables|Default|GetWispAbility)
          (CallFunction|SetWisp)
          (CallFunction|RefreshItem)
          (Variables|Default|SetWispAbility false)))
      (:then_2
        (if (Variables|Default|GetWingRabitAbility)
          (CallFunction|SetWingRabbit)
          (CallFunction|RefreshItem)
          (Variables|Default|SetWingRabitAbility false))))))

(event Input|AxisEvents|InputAxisMoveForward
  (params (AxisValue :type Float%20%28single-precision%29))
  (bind _returnvalue (Game|Player|GetPlayerPawn 0))
  ;[1 1 1] Controller
  (Pawn|Input|AddMovementInput _returnvalue (Math|Vector|GetForwardVector (Pawn|GetControlRotation _returnvalue :!class /Script/Engine.Pawn)) AxisValue false))

(event Input|AxisEvents|InputAxisMoveRight
  (params (AxisValue :type Float%20%28single-precision%29))
  (bind _returnvalue (Game|Player|GetPlayerPawn 0))
  ;[1 1 1] Controller
  (Pawn|Input|AddMovementInput _returnvalue (Math|Vector|GetRightVector (Pawn|GetControlRotation _returnvalue :!class /Script/Engine.Pawn)) AxisValue false))

(event Input|AxisEvents|InputAxisForcus
  (params (AxisValue :type Float%20%28single-precision%29))
  (bind _springarm (Variables|Default|GetSpringArm))
  ;[1 1 1] Comment
  (Variables|/Script/Engine.SpringArmComponent|SetTargetArmLength _springarm (+ (Variables|/Script/Engine.SpringArmComponent|GetTargetArmLength _springarm) (* AxisValue -1e+01))))

(event Input|AxisEvents|InputAxisTurn
  (params (AxisValue :type Float%20%28single-precision%29))
  ;[1 1 1] Controller
  (Pawn|Input|AddControllerYawInput (Game|GetPlayerCharacter 0) AxisValue))

(fn ConstructionScript)

(fn AddScore
  (bind _output_get (Variables|Default|SetScore (+ (Variables|Default|GetScore) (Variables|Default|Getscore_slime))))
  (Transformation|SetWorldScale3D (Variables|Character|GetMesh) (+ (Variables|Default|Getmagnification_vector) (* (/ _output_get (Variables|Default|Getmagnification_score)) (Variables|Default|Getmagnification)))))

(fn AddScoreWolf
  (bind _output_get (Variables|Default|SetScore (+ (Variables|Default|GetScore) (Variables|Default|Getscore_wolf))))
  (Transformation|SetWorldScale3D (Variables|Character|GetMesh) (+ (Variables|Default|Getmagnification_vector) (* (/ _output_get (Variables|Default|Getmagnification_score)) (Variables|Default|Getmagnification)))))

(fn AddItem
  (bind _actortrace (Variables|Default|GetActorTrace))
  (bind _actortrace_2 (Variables|Default|GetActorTrace))
  (bind (_asbp_wolf _bsuccess) (Utilities|Casting|CastToBP_Wolf _actortrace))
  (bind (_aswing_rabbit _bsuccess_2) (Utilities|Casting|CastToWingRabbit _actortrace))
  (bind (_asbp_whisp _bsuccess_3) (Utilities|Casting|CastToBP_Whisp _actortrace))
  (bind (_aswing_rabbit_2 _bsuccess_4) (Utilities|Casting|CastToWingRabbit _actortrace_2))
  (bind (_asbp_wolf_2 _bsuccess_5) (Utilities|Casting|CastToBP_Wolf _actortrace_2))
  (bind (_asbp_whisp_2 _bsuccess_6) (Utilities|Casting|CastToBP_Whisp _actortrace_2))
  (if (Variables|Default|GetHaveItem?)
    (Variables|Default|SetWispAbility false)
    (Variables|Default|SetWolfAbility false)
    (Variables|Default|SetWingRabitAbility false)
    (Utilities|Array|SetArrayElem :TargetArray (Variables|Default|GetInventory) :Index (Variables|Default|GetSlotIndex))
    (CallFunction|RefreshItem)
    (Utilities|FlowControl|Sequence
      (:then_0
        (if _bsuccess
          (Utilities|Array|Add (Variables|Default|GetInventory) (Variables|/Game/BluePrints/BP_Inventory/Inventory/test.test_C|GetItemData _asbp_wolf))
          (if _bsuccess
            (Variables|Default|SetWolfAbility true)
            (Variables|Default|SetHaveItem? true :!label _label)
            (return))))
      (:then_1
        (if _bsuccess_3
          (Utilities|Array|Add (Variables|Default|GetInventory) (Variables|/Game/BluePrints/BP_Inventory/Inventory/test.test_C|GetItemData _asbp_whisp))
          (if _bsuccess_3
            (Variables|Default|SetWispAbility true)
            (goto _label))))
      (:then_2
        (if _bsuccess_2
          (Utilities|Array|Add (Variables|Default|GetInventory) (Variables|/Game/BluePrints/BP_Inventory/Inventory/test.test_C|GetItemData _aswing_rabbit))
          (if _bsuccess_2
            (Variables|Default|SetWingRabitAbility true)))))
    (else
      (Utilities|FlowControl|Sequence
        (:then_0
          (if _bsuccess_5
            (Utilities|Array|Add (Variables|Default|GetInventory) (Variables|/Game/BluePrints/BP_Inventory/Inventory/test.test_C|GetItemData _asbp_wolf_2))
            (if _bsuccess_5
              (Variables|Default|SetWolfAbility true)
              (Variables|Default|SetHaveItem? true :!label _label_2)
              (return))))
        (:then_1
          (if _bsuccess_6
            (Utilities|Array|Add (Variables|Default|GetInventory) (Variables|/Game/BluePrints/BP_Inventory/Inventory/test.test_C|GetItemData _asbp_whisp_2))
            (if _bsuccess_6
              (Variables|Default|SetWispAbility true)
              (goto _label_2))))
        (:then_2
          (if _bsuccess_4
            (Utilities|Array|Add (Variables|Default|GetInventory) (Variables|/Game/BluePrints/BP_Inventory/Inventory/test.test_C|GetItemData _aswing_rabbit_2))
            (if _bsuccess_4
              (Variables|Default|SetWingRabitAbility true)
              (goto _label_2))))))))

(fn SetWolf
  (Variables|/Script/Engine.CharacterMovementComponent|SetMaxWalkSpeed (Variables|Character|GetCharacterMovement) (Variables|Default|Getspeed))
  (return))

(fn AddScoreWisp
  (bind _output_get (Variables|Default|SetScore (+ (Variables|Default|GetScore) (Variables|Default|GetScoreWisp))))
  (Transformation|SetWorldScale3D (Variables|Character|GetMesh) (+ (Variables|Default|Getmagnification_vector) (* (/ _output_get (Variables|Default|Getmagnification_score)) (Variables|Default|Getmagnification)))))

(fn SetWisp
  (Effects|SpawnEmitteratLocation "/Game/Goto/Whisp/WhispParticle.WhispParticle" (Transformation|GetWorldLocation (Variables|Character|GetMesh))))

(fn RefreshItem
  (bind _output_get (Variables|Default|SetItemData (Utilities|Array|Get(acopy) (Variables|Default|GetInventory) (Variables|Default|GetSlotIndex))))
  (if (<= (.quality _output_get) 0)
    (Variables|Default|SetItemData "")
    (Utilities|Array|SetArrayElem :TargetArray (Variables|Default|GetInventory) :Index (Variables|Default|GetSlotIndex))
    (return)))

(fn AddScoreLizard
  (bind _output_get (Variables|Default|SetScore (+ (Variables|Default|GetScore) (Variables|Default|GetScoreLizard))))
  (Transformation|SetWorldScale3D (Variables|Character|GetMesh) (+ (Variables|Default|Getmagnification_vector) (* (/ _output_get (Variables|Default|Getmagnification_score)) (Variables|Default|Getmagnification)))))

(fn AddScoreWingRabbit
  (bind _output_get (Variables|Default|SetScore (+ (Variables|Default|GetScore) (Variables|Default|GetScoreWingRabbit))))
  (Transformation|SetWorldScale3D (Variables|Character|GetMesh) (+ (Variables|Default|Getmagnification_vector) (* (/ _output_get (Variables|Default|Getmagnification_score)) (Variables|Default|Getmagnification)))))

(fn SetWingRabbit
  (bind _charactermovement (Variables|Character|GetCharacterMovement))
  (Variables|/Script/Engine.CharacterMovementComponent|SetJumpZVelocity _charactermovement 1.6e+03)
  (Character|Jump (Game|GetPlayerCharacter 0))
  (Variables|/Script/Engine.CharacterMovementComponent|SetJumpZVelocity _charactermovement 8e+02))