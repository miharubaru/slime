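; Slime character Blueprint that tracks a score and grows its mesh as that score rises.
; BeginPlay sets the point values for grass and wolves, plus the growth step and rate.
; AddScore and AddScoreWolf each add their points, then set the mesh's world scale to a base vector plus a uniform bonus derived from the accumulated score.
; Nothing in this Blueprint calls either function.
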(event EventBeginPlay
  (Utilities|FlowControl|Sequence ; 敵のスコア/スライムの巨大化数値
    (:then_0
      (Variables|Default|Setscore_slime 1) ; 草のスコア
      (Variables|Default|Setscore_wolf 5) ; ウルフのスコア/新しい敵はこの右に継ぎ足しok
    )
    (:then_1
      (Variables|Default|Setmagnification_score 5) ; スライムの大きくなるscoreの設定
      (Variables|Default|Setmagnification 0.1) ; スライムの大きくなる倍率
      (Variables|Default|Setmagnification_vector "1.000000,1.000000,1.000000") ; 巨大化に使うVector値。いじらなくてヨシ!
    )))

(fn ConstructionScript)

(fn AddScore
  (bind _output_get (Variables|Default|SetScore (+ (Variables|Default|GetScore) (Variables|Default|Getscore_slime))))
  (Transformation|SetWorldScale3D (Variables|Character|GetMesh) (+ (Variables|Default|Getmagnification_vector) (* (/ _output_get (Variables|Default|Getmagnification_score)) (Variables|Default|Getmagnification)))))

(fn AddScoreWolf
  (bind _output_get (Variables|Default|SetScore (+ (Variables|Default|GetScore) (Variables|Default|Getscore_wolf))))
  (Transformation|SetWorldScale3D (Variables|Character|GetMesh) (+ (Variables|Default|Getmagnification_vector) (* (/ _output_get (Variables|Default|Getmagnification_score)) (Variables|Default|Getmagnification)))))