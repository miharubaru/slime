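; Player 2's slime character in local multiplayer, with its own movement, camera zoom, score-costing jump and inventory widget.
; AddScore functions for grass and creatures enlarge the mesh; touching a larger BP_Character hides this slime and opens the result level.
; AddItem stores Wolf, Wisp or WingRabbit abilities, which MultiAbility consumes for a speed burst, particle effect or high jump.
; Tick drives a FlipFlop that creates and removes the inventory widget on alternate frames.
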(event OnComponentBeginOverlap(Sphere)
  (params (OverlappedComponent :type Primitive%20Component%20Object%20Reference) (OtherActor :type Actor%20Object%20Reference) (OtherComp :type Primitive%20Component%20Object%20Reference) (OtherBodyIndex :type Integer) (bFromSweep :type Boolean) (SweepResult :type Hit%20Result%20Structure%20%28by%20ref%29))
  (bind _returnvalue (Game|GetPlayerCharacter 0))
  (bind _asbp_character (Utilities|Casting|CastToBP_Character _returnvalue))
  (if (.bSuccess (Utilities|Casting|CastToBP_Character OtherActor))
    (Utilities|FlowControl|Sequence
      (:then_0
        (bind _output_get (Variables|Default|SetSlimeScale_2 (.z (Transformation|GetWorldScale (Variables|Character|GetMesh))))))
      (:then_1
        (bind _output_get_2 (Variables|/Game/BluePrints/BP_Character/BP_Character.BP_Character_C|SetSlimeScale _asbp_character (.z (Transformation|GetWorldScale (Variables|/Script/Engine.Character|GetMesh _asbp_character)))))))
    (if (< _output_get _output_get_2)
      (Rendering|SetVisibility (Variables|Character|GetMesh) false false)
      (Rendering|SetVisibility (Variables|Default|GetSphere) false false)
      (Rendering|SetVisibility (Variables|Collision|GetCapsuleComponent) false false)
      (Game|OpenLevel(byName) "result"))))

(event EventBeginPlay
  (Utilities|FlowControl|Sequence
    (:then_0
      (Variables|Default|Setscore_grass_2 1)
      (Variables|Default|SetScoreWisp2 5)
      (Variables|Default|Setscore_wolf_2 5)
      (Variables|Default|SetScoreLizard 5)
      (Variables|Default|SetScore_WingRabbitt 10))
    (:then_1
      (Variables|Default|Setmagnification_score_2 30) ; スライムの大きくなるscoreの設定
      (Variables|Default|Setmagnification_2 0.2) ; スライムの大きくなる倍率
      (Variables|Default|Setmagnification_vector_2 "1.000000,1.000000,1.000000"))))

(event EventTick
  (params (DeltaSeconds :type Float%20%28single-precision%29))
  (bind _returnvalue (Game|GetPlayerController 1))
  ;[1 1 1] Player2
  ;;[1 1 1] Inventory
  (Utilities|FlowControl|FlipFlop
    (:A
      (bind _returnvalue_2 (UserInterface|CreateWidget "/Game/BluePrints/BP_Inventory/Inventory/Inventory_2.Inventory_2_C" _returnvalue))
      (bind _output_get (Variables|Default|SetInventoryRef _returnvalue_2))
      (UserInterface|Viewport|AddtoViewport _output_get 0)
      (Variables|/Script/Engine.PlayerController|SetbShowMouseCursor _returnvalue true)
      (Input|SetInputModeGameandUI _returnvalue 0 "DoNotLock" true))
    (:B
      (Widget|RemovefromParent (Variables|Default|GetInventoryRef))
      (Variables|/Script/Engine.PlayerController|SetbShowMouseCursor _returnvalue false)
      (Input|SetInputModeGameOnly _returnvalue))))

(event Input|ActionEvents|InputActionMultiAbility
  (params (Key :type Key%20Structure :default "None"))
  ;[1 1 1] Player2
  ;;[1 1 1] Ability
  (:Pressed
    (Utilities|FlowControl|Sequence
      (:then_0
        (if (Variables|Default|GetWolfAbirity2)
          (CallFunction|SetWolf)
          (Utilities|FlowControl|Delay 3.0)
          (Variables|/Script/Engine.CharacterMovementComponent|SetMaxWalkSpeed (Variables|Character|GetCharacterMovement) 6e+02)
          (CallFunction|RefresshItem)
          (Variables|Default|SetWolfAbirity2 false)))
      (:then_1
        (if (Variables|Default|GetWispAbility2)
          (CallFunction|SetWisp)
          (CallFunction|RefresshItem)
          (Variables|Default|SetWispAbility2 false)))
      (:then_2
        (if (Variables|Default|GetWingRabbitAbility)
          (CallFunction|SetWingRabbit)
          (CallFunction|RefresshItem)
          (Variables|Default|SetWingRabbitAbility false))))))

(event Input|ActionEvents|InputActionMultiJump
  (params (Key :type Key%20Structure :default "None"))
  ;[1 1 1] Player2
  ;;[1 1 1] MultiControl
  (:Pressed
    (Utilities|FlowControl|Delay 0.5)
    (Character|Jump (Game|GetPlayerCharacter 1))
    (Utilities|FlowControl|Delay 1.5)
    (Variables|Default|SetScore (- (Variables|Default|GetScore) (Variables|Default|GetJumoScore)))))

(event Input|AxisEvents|InputAxisMultiForcus
  (params (AxisValue :type Float%20%28single-precision%29))
  (bind _returnvalue (Game|GetPlayerCharacter 1))
  (bind _asbp_character_02 (Utilities|Casting|CastToBP_Character_02 _returnvalue))
  (bind _springarm (Variables|BP_Character_02_C|GetSpringArm _asbp_character_02))
  ;[1 1 1] Player2
  ;;[1 1 1] Camera
  (Variables|/Script/Engine.SpringArmComponent|SetTargetArmLength _springarm (+ (Variables|/Script/Engine.SpringArmComponent|GetTargetArmLength _springarm) (* AxisValue -1e+01))))

(event Input|AxisEvents|InputAxisMultiMoveForward
  (params (AxisValue :type Float%20%28single-precision%29))
  (bind _returnvalue (Game|GetPlayerCharacter 1))
  ;[1 1 1] Player2
  ;;[1 1 1] MultiControl
  (Pawn|Input|AddMovementInput _returnvalue (Math|Vector|GetForwardVector (Pawn|GetControlRotation _returnvalue :!class /Script/Engine.Pawn)) AxisValue false))

(event Input|AxisEvents|InputAxisMultiRightForward
  (params (AxisValue :type Float%20%28single-precision%29))
  (bind _returnvalue (Game|GetPlayerCharacter 1))
  ;[1 1 1] Player2
  ;;[1 1 1] MultiControl
  (Pawn|Input|AddMovementInput _returnvalue (Math|Vector|GetRightVector (Pawn|GetControlRotation _returnvalue :!class /Script/Engine.Pawn)) AxisValue false))

(event Input|AxisEvents|InputAxisMultiTurn
  (params (AxisValue :type Float%20%28single-precision%29))
  ;[1 1 1] Player2
  ;;[1 1 1] MultiControl
  (Pawn|Input|AddControllerYawInput (Game|GetPlayerCharacter 1) AxisValue))

(fn ConstructionScript)

(fn AddScore
  (bind _output_get (Variables|Default|SetScore (+ (Variables|Default|GetScore) (Variables|Default|Getscore_grass_2))))
  (Transformation|SetWorldScale3D (Variables|Character|GetMesh) (+ (Variables|Default|Getmagnification_vector_2) (* (/ _output_get (Variables|Default|Getmagnification_score_2)) (Variables|Default|Getmagnification_2)))))

(fn AddScoreWolf
  (bind _output_get (Variables|Default|SetScore (+ (Variables|Default|GetScore) (Variables|Default|Getscore_wolf_2))))
  (Transformation|SetWorldScale3D (Variables|Character|GetMesh) (+ (Variables|Default|Getmagnification_vector_2) (* (/ _output_get (Variables|Default|Getmagnification_score_2)) (Variables|Default|Getmagnification_2)))))

(fn AddItem
  (bind _actortrace (Variables|Default|GetActorTrace))
  (bind _actortrace_2 (Variables|Default|GetActorTrace))
  (bind (_asbp_wolf _bsuccess) (Utilities|Casting|CastToBP_Wolf _actortrace_2))
  (bind (_asbp_wolf_2 _bsuccess_2) (Utilities|Casting|CastToBP_Wolf _actortrace))
  (bind (_asbp_whisp _bsuccess_3) (Utilities|Casting|CastToBP_Whisp _actortrace))
  (bind (_asbp_whisp_2 _bsuccess_4) (Utilities|Casting|CastToBP_Whisp _actortrace_2))
  (bind (_aswing_rabbit _bsuccess_5) (Utilities|Casting|CastToWingRabbit _actortrace))
  (bind (_aswing_rabbit_2 _bsuccess_6) (Utilities|Casting|CastToWingRabbit _actortrace_2))
  (if (Variables|Default|GetHaveItem?)
    (Variables|Default|SetWolfAbirity2 false)
    (Variables|Default|SetWispAbility2 false)
    (Variables|Default|SetWingRabbitAbility false)
    (Utilities|Array|SetArrayElem :TargetArray (Variables|Default|GetInventory) :Index (Variables|Default|GetInventorySlit))
    (CallFunction|RefresshItem)
    (Utilities|FlowControl|Sequence
      (:then_0
        (if _bsuccess_2
          (Utilities|Array|Add (Variables|Default|GetInventory) (Variables|/Game/BluePrints/BP_Inventory/Inventory/test.test_C|GetItemData _asbp_wolf_2))
          (if _bsuccess_2
            (Variables|Default|SetWolfAbirity2 true)
            (Variables|Default|SetHaveItem? true :!label _label)
            (return))))
      (:then_1
        (if _bsuccess_3
          (Utilities|Array|Add (Variables|Default|GetInventory) (Variables|/Game/BluePrints/BP_Inventory/Inventory/test.test_C|GetItemData _asbp_whisp))
          (if _bsuccess_3
            (Variables|Default|SetWispAbility2 true)
            (goto _label))))
      (:then_2
        (if _bsuccess_5
          (Utilities|Array|Add (Variables|Default|GetInventory) (Variables|/Game/BluePrints/BP_Inventory/Inventory/test.test_C|GetItemData _aswing_rabbit))
          (if _bsuccess_5
            (Variables|Default|SetWingRabbitAbility true)
            (goto _label)))))
    (else
      (Utilities|FlowControl|Sequence
        (:then_0
          (if _bsuccess
            (Utilities|Array|Add (Variables|Default|GetInventory) (Variables|/Game/BluePrints/BP_Inventory/Inventory/test.test_C|GetItemData _asbp_wolf))
            (if _bsuccess
              (Variables|Default|SetWolfAbirity2 true)
              (Variables|Default|SetHaveItem? true :!label _label_2)
              (return))))
        (:then_1
          (if _bsuccess_4
            (Utilities|Array|Add (Variables|Default|GetInventory) (Variables|/Game/BluePrints/BP_Inventory/Inventory/test.test_C|GetItemData _asbp_whisp_2))
            (if _bsuccess_4
              (Variables|Default|SetWispAbility2 true)
              (goto _label_2))))
        (:then_2
          (if _bsuccess_6
            (Utilities|Array|Add (Variables|Default|GetInventory) (Variables|/Game/BluePrints/BP_Inventory/Inventory/test.test_C|GetItemData _aswing_rabbit_2))
            (if _bsuccess_6
              (Variables|Default|SetWingRabbitAbility true)
              (goto _label_2))))))))

(fn SetWolf
  (Variables|/Script/Engine.CharacterMovementComponent|SetMaxWalkSpeed (Variables|Character|GetCharacterMovement) 5e+03)
  (return))

(fn AddScoreWisp
  (bind _output_get (Variables|Default|SetScoreWisp2 (+ (Variables|Default|GetScore) (Variables|Default|GetScoreWisp2))))
  (Transformation|SetWorldScale3D (Variables|Character|GetMesh) (+ (Variables|Default|Getmagnification_vector_2) (* (/ _output_get (Variables|Default|Getmagnification_score_2)) (Variables|Default|Getmagnification_2)))))

(fn SetWisp
  (Effects|SpawnEmitteratLocation "/Game/Goto/Whisp/WhispParticle.WhispParticle" (Transformation|GetWorldLocation (Variables|Character|GetMesh))))

(fn RefresshItem
  (bind _output_get (Variables|Default|SetItemData (Utilities|Array|Get(acopy) (Variables|Default|GetInventory) (Variables|Default|GetInventorySlit))))
  (if (<= (.quality _output_get) 0)
    (Variables|Default|SetItemData "")
    (Utilities|Array|SetArrayElem :TargetArray (Variables|Default|GetInventory) :Index (Variables|Default|GetInventorySlit))
    (return)))

(fn AddScoreLizard
  (bind _output_get (Variables|Default|SetScore (+ (Variables|Default|GetScore) (Variables|Default|GetScoreLizard))))
  (Transformation|SetWorldScale3D (Variables|Character|GetMesh) (+ (Variables|Default|Getmagnification_vector_2) (* (/ _output_get (Variables|Default|Getmagnification_score_2)) (Variables|Default|Getmagnification_2)))))

(fn AddScoreWingRabbit
  (bind _output_get (Variables|Default|SetScore (+ (Variables|Default|GetScore) (Variables|Default|GetScore_WingRabbitt))))
  (Transformation|SetWorldScale3D (Variables|Character|GetMesh) (+ (Variables|Default|Getmagnification_vector_2) (* (/ _output_get (Variables|Default|Getmagnification_score_2)) (Variables|Default|Getmagnification_2)))))

(fn SetWingRabbit
  (Variables|/Script/Engine.CharacterMovementComponent|SetJumpZVelocity (Variables|Character|GetCharacterMovement) 3e+03)
  (Character|Jump (Game|GetPlayerCharacter 1)))